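; BaseAI is the base AI pawn for a ball game, handling ball pickup contact and visual state.
; On overlap, it checks the first overlapping BaseBall and, if possessable, passes it to BaseAIController's AIBallPickup.
; Three events swap the skeletal mesh's placeholder material for normal, stunned and stealing states.
; The construction script caches the mesh for socket use and records the start transform.
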(event `self.ReceiveActorBeginOverlap`
  (params (OtherActor :type "Actor Object Reference"))
  (bind _overlappingactors (`self.GetOverlappingActors` "/Game/Blueprints/Ball/BaseBall.BaseBall_C"))
  ;[1 1 1 1 28] Ball Overlap
  (if (!= (`KismetArrayLibrary.Array_Length` _overlappingactors) 0)
    (bind _asbase_ball (cast `/Game/Blueprints/Ball/BaseBall` (`|GetArrayItem` _overlappingactors)))
    (if (`/Game/Blueprints/Ball/BaseBall.bPossessable` _asbase_ball)
      (bind _asbase_aicontroller (cast `/Game/Blueprints/AI/BaseAIController` (`AIBlueprintHelperLibrary.GetAIController` self)))
      (`/Game/Blueprints/AI/BaseAIController.AIBallPickup` _asbase_aicontroller _asbase_ball))))

(event `SetMaterialNormal`
  (`PrimitiveComponent.SetMaterial` (`self.AISkeletalMesh`) 0 "/Game/Materials/Custom/MI_Placeholder_AI.MI_Placeholder_AI") ; Normal
)

(event `SetMaterialStunned`
  (`PrimitiveComponent.SetMaterial` (`self.AISkeletalMesh`) 0 "/Game/Materials/Custom/MI_Placeholder_AI_Stunned.MI_Placeholder_AI_Stunned") ; Stunned
)

(event `SetMaterialStealing`
  (`PrimitiveComponent.SetMaterial` (`self.AISkeletalMesh`) 0 "/Game/Materials/Custom/MI_Placeholder_AI_Stealing.MI_Placeholder_AI_Stealing") ; Stealing
)

(fn `UserConstructionScript`
  ;[1 1 1 1 28] Skeletal Mesh Reference (for sockets)
  (set `self.AISkeletalMesh` (`self.Mesh`))
  ;[1 1 1 1 28] Start Location
  (set `self.StartTransform` (`self.GetTransform` self)))