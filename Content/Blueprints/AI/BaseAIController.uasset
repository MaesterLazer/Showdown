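; AI controller for a basketball opponent that runs a behavior tree and provides steal, block, stun and ball pickup actions against the player.
; On begin play it caches the ball, player, hoop and its pawn's detectors.
; Steal and block check detector overlaps for a player with possession, gated by blackboard flags with randomized cooldowns.
; Blocks fire once per active shot, launching the pawn along the ball-to-hoop direction.
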(event `self.ReceiveBeginPlay`
  ;[1 1 1 1 28] Begin Play
  (`self.DefineTheBall`)
  (`self.DefineThePlayer`)
  (`self.DefineMyAIMySkeleton`)
  (`self.DefineTheHoop`)
  (`self.RunBehaviorTree` (`self.BehaviorTree`))
  (`self.StealCooldown`)
  (`self.BlockCooldown`))

(event `DefineTheBall`
  ;[1 1 1 1 28] Begin Play
  (bind _outactors (`GameplayStatics.GetAllActorsOfClass` "/Game/Blueprints/BaseBall.BaseBall_C"))
  (set `self.TheBall` (`|GetArrayItem` _outactors)))

(event `DefineThePlayer`
  ;[1 1 1 1 28] Begin Play
  (bind _outactors (`GameplayStatics.GetAllActorsOfClass` "/Game/Blueprints/Player/BaseCharacter.BaseCharacter_C"))
  (bind _output_get (set `self.ThePlayer` (`|GetArrayItem` _outactors)))
  (set `self.PlayerStunDetector` (`/Game/Blueprints/Player/BaseCharacter.StunDetector` _output_get)))

(event `DefineMyAIMySkeleton`
  ;[1 1 1 1 28] Begin Play
  (bind _asbase_ai (cast `/Game/Blueprints/AI/BaseAI` (`self.K2_GetPawn`)))
  (bind _output_get (set `self.MyAiCharacter` _asbase_ai))
  (set `self.MySkeletalMesh` (`/Game/Blueprints/AI/BaseAI.AISkeletalMesh` _output_get))
  (set `self.MyStunDetector` (`/Game/Blueprints/AI/BaseAI.StunDetector` (`self.MyAiCharacter`)))
  (set `self.MyBlockDetector` (`/Game/Blueprints/AI/BaseAI.BlockDetector` (`self.MyAiCharacter`))))

(event `DefineTheHoop`
  ;[1 1 1 1 28] Begin Play
  (bind _outactors (`GameplayStatics.GetAllActorsOfClass` "/Game/Blueprints/BaseHoop.BaseHoop_C"))
  (bind _output_get (set `self.TheHoop` (`|GetArrayItem` _outactors)))
  (set `self.HoopTarget` (`self.K2_GetActorLocation` _output_get)))

(event `StunMe`
  (params (StunDelay :type "Float (double-precision)"))
  ;[1 1 1 1 28] Stun
  (`BlackboardComponent.SetValueAsBool` (`AIBlueprintHelperLibrary.GetBlackboard` self) (`self.StunKey`) true)
  (`KismetSystemLibrary.Delay` StunDelay)
  (`KismetSystemLibrary.PrintString` "AI no longer stunned")
  (`BlackboardComponent.SetValueAsBool` (`AIBlueprintHelperLibrary.GetBlackboard` self) (`self.StunKey`) false))

(event `Steal`
  (bind _overlappingactors (`PrimitiveComponent.GetOverlappingActors` (`self.MyStunDetector`) "/Game/Blueprints/Player/BaseCharacter.BaseCharacter_C"))
  ;[1 1 1 1 28] Steal
  (if (`BlackboardComponent.GetValueAsBool` (`AIBlueprintHelperLibrary.GetBlackboard` self) (`self.StealKey`))
    (if (> (`KismetArrayLibrary.Array_Length` _overlappingactors) 0)
      (bind _asbase_character (cast `/Game/Blueprints/Player/BaseCharacter` (`|GetArrayItem` _overlappingactors)))
      (bind _asbase_character_controller (cast `/Game/Blueprints/Player/BaseCharacterController` (`Pawn.GetController` _asbase_character)))
      (if (`/Game/Blueprints/Player/BaseCharacterController.bHasPossession` _asbase_character_controller)
        (`self.SetCanSteal` false)
        (`/Game/Blueprints/Player/BaseCharacterController.StealMe` _asbase_character_controller self)
        (`self.StealCooldown`)))))

(event `SetCanSteal`
  (params (BoolValue :type Boolean))
  ;[1 1 1 1 28] Steal
  (`BlackboardComponent.SetValueAsBool` (`AIBlueprintHelperLibrary.GetBlackboard` self) (`self.StealKey`) BoolValue))

(event `StealCooldown`
  ;[1 1 1 1 28] Steal
  (`KismetSystemLibrary.Delay` (`KismetMathLibrary.RandomFloatInRange` (`self.StealCooldownTimeMin`) (`self.StealCooldownTimeMax`)))
  (`self.SetCanSteal` true))

(event `BlockAttempt`
  (bind _overlappingactors (`PrimitiveComponent.GetOverlappingActors` (`self.MyBlockDetector`) "/Game/Blueprints/Player/BaseCharacter.BaseCharacter_C"))
  ;[1 1 1 1 28] Block
  (if (`BlackboardComponent.GetValueAsBool` (`AIBlueprintHelperLibrary.GetBlackboard` self) (`self.BlockKey`))
    (if (> (`KismetArrayLibrary.Array_Length` _overlappingactors) 0)
      (bind _asbase_character (cast `/Game/Blueprints/Player/BaseCharacter` (`|GetArrayItem` _overlappingactors)))
      (bind _asbase_character_controller (cast `/Game/Blueprints/Player/BaseCharacterController` (`Pawn.GetController` _asbase_character)))
      (if (`/Game/Blueprints/Player/BaseCharacterController.bHasPossession` _asbase_character_controller)
        (if (`/Game/Blueprints/Player/BaseCharacterController.bShotActive` _asbase_character_controller)
          (`/Engine/EditorBlueprintResources/StandardMacros.DoOnce` false :!label _label
            (:`Completed`
              (`self.SetCanBlock` false)
              (`self.BlockCooldown`)
              (`self.Block`)))
          (else
            (goto _label :!via `Reset`)))))))

(event `Block`
  ;[1 1 1 1 28] Block
  (`KismetSystemLibrary.PrintString` "Blocking")
  (`self.BlockVector`))

(event `SetCanBlock`
  (params (`Bool Value` :type Boolean))
  ;[1 1 1 1 28] Block
  (`BlackboardComponent.SetValueAsBool` (`AIBlueprintHelperLibrary.GetBlackboard` self) (`self.BlockKey`) `Bool Value`))

(event `BlockVector`
  ;[1 1 1 1 28] Block
  (`self.BlockJump` (* (`KismetMathLibrary.GetDirectionUnitVector` (`self.K2_GetActorLocation` (`self.TheBall`)) (`self.K2_GetActorLocation` (`self.TheHoop`))) 30.0)))

(event `BlockJump`
  (params (LaunchVelocity :type "Vector Structure"))
  ;[1 1 1 1 28] Block
  (`Character.LaunchCharacter` (`self.MyAiCharacter`) (* LaunchVelocity (`self.BlockFactor`)) false false))

(event `BlockCooldown`
  ;[1 1 1 1 28] Block
  (`KismetSystemLibrary.Delay` (`KismetMathLibrary.RandomFloatInRange` (`self.BlockCooldownTimeMin`) (`self.BlockCooldownTimeMax`)))
  (`self.SetCanBlock` true))

(event `BallPickup`
  (params (Ball :type "/Game/Blueprints/BaseBall Object Reference"))
  ;[1 1 1 1 24] Ball Pickup
  (if (not (`/Game/Blueprints/BaseBall.bIsShot` Ball))
    (`BlackboardComponent.SetValueAsBool` (`AIBlueprintHelperLibrary.GetBlackboard` self) (`KismetStringLibrary.Conv_StringToName` "bSwitchSides") true)))

(fn `UserConstructionScript`)