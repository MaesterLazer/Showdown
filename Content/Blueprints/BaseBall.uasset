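; Basketball actor that can be picked up, shot, tipped and stolen, targeting the level's hoop found on BeginPlay.
; State events switch collision profile, physics and possessability as the ball attaches to or detaches from its holder.
; Shots apply a supplied launch velocity, with a selection choosing advantage tip or swish.
; Hoop or character hits free the ball, arcing advantage rim tips toward the hoop, while steals pop it loose randomly.
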(event `self.ReceiveBeginPlay`
  ;[1 1 1 1 28] Startup
  (`self.DefineTheHoopTarget`))

(event `DefineTheHoopTarget`
  ;[1 1 1 1 28] Startup
  (bind _outactors (`GameplayStatics.GetAllActorsOfClass` "/Game/Blueprints/BaseHoop.BaseHoop_C"))
  (set `self.HoopTarget` (`self.K2_GetActorLocation` (`|GetArrayItem` _outactors)))
  (bind _returnvalue (`KismetArrayLibrary.Array_Length` _outactors))
  (if (!= _returnvalue 0)
    (if (> _returnvalue 1)
      (`KismetSystemLibrary.PrintString` "More than 1 hoop in scene." false))
    (else
      (`KismetSystemLibrary.PrintString` "No hoops in scene." false))))

(event `StateFree`
  ;[1 1 1 1 28] States
  (`PrimitiveComponent.SetCollisionProfileName` (`self.StaticMesh`) "BallFree")
  (`PrimitiveComponent.SetSimulatePhysics` (`self.StaticMesh`) true)
  (set `PrimitiveComponent.bGenerateOverlapEvents` true (`self.StaticMesh`))
  (set `self.Possessable` true)
  (set `self.DebugBallState` "Free"))

(event `StatePossessed`
  ;[1 1 1 1 28] States
  (`PrimitiveComponent.SetSimulatePhysics` (`self.StaticMesh`) false)
  (`PrimitiveComponent.SetCollisionProfileName` (`self.StaticMesh`) "BallPossessed")
  (set `self.Possessable` false)
  (set `self.DebugBallState` "Posessed"))

(event `StateShot`
  ;[1 1 1 1 28] States
  (`PrimitiveComponent.SetCollisionProfileName` (`self.StaticMesh`) "BallFree")
  (`PrimitiveComponent.SetSimulatePhysics` (`self.StaticMesh`) true)
  (set `PrimitiveComponent.bGenerateOverlapEvents` false (`self.StaticMesh`)) ; Might not be necessary
  (set `self.Possessable` false)
  (set `self.DebugBallState` "Shot"))

(event `StateStolen`
  ;[1 1 1 1 28] States
  (`PrimitiveComponent.SetCollisionProfileName` (`self.StaticMesh`) "BallStolen")
  (`PrimitiveComponent.SetSimulatePhysics` (`self.StaticMesh`) true)
  (set `PrimitiveComponent.bGenerateOverlapEvents` true (`self.StaticMesh`))
  (set `self.Possessable` false)
  (set `self.DebugBallState` "Stolen"))

(event `StateSwish`
  ;[1 1 1 1 28] States
  (`PrimitiveComponent.SetCollisionProfileName` (`self.StaticMesh`) "BallSwish")
  (`PrimitiveComponent.SetSimulatePhysics` (`self.StaticMesh`) true)
  (set `self.DebugBallState` "Swish"))

(event `StateReset`
  ;[1 1 1 1 28] States
  (`PrimitiveComponent.SetCollisionProfileName` (`self.StaticMesh`) "BallFree")
  (`PrimitiveComponent.SetSimulatePhysics` (`self.StaticMesh`) true)
  (set `self.DebugBallState` "Reset"))

(event `AttachBallTo`
  (params (Parent :type "SceneComponent Object Reference") (SocketName :type Name))
  ;[1 1 1 1 28] Attach
  (`self.K2_AttachToComponent` Parent SocketName "SnapToTarget" "KeepRelative" "KeepRelative" false))

(event `PickUpBall`
  (params (Parent :type "SceneComponent Object Reference") (SocketName :type Name))
  ;[1 1 1 1 28] Pick Up
  (if (`self.Possessable`)
    (`self.StatePossessed`)
    (`self.AttachBallTo` Parent SocketName)))

(event `ShootBall`
  (params (LaunchVelocity :type "Vector Structure") (Selection :type Integer))
  ;[1 1 1 1 28] Shoot
  (switch `int` Selection
    (:`0`
      (set `self.AdvantageTip` false)
      (`self.StateShot` :!label _label))
    (:`1`
      (set `self.AdvantageTip` true)
      (goto _label))
    (:`2`
      (`self.StateSwish`)))
  (`PrimitiveComponent.SetPhysicsLinearVelocity` (`self.StaticMesh`) LaunchVelocity false "None")
  (`self.K2_DetachFromActor` "KeepRelative"))

(event `self.StaticMesh.OnComponentHit`
  (params (HitComponent :type "PrimitiveComponent Object Reference") (OtherActor :type "Actor Object Reference") (OtherComp :type "PrimitiveComponent Object Reference") (NormalImpulse :type "Vector Structure") (Hit :type "HitResult Structure (by ref)"))
  (bind _returnvalue (`GameplayStatics.GetObjectClass` OtherActor))
  ;[1 1 1 1 28] Mid-Shot Collision (Hoop/Person/Other)
  (if (`self.Possessable`)
    _
    (elif (== _returnvalue "/Game/Blueprints/BaseHoop.BaseHoop_C")
      (`self.TipBall` :!label _label_2)
      (elif (== _returnvalue "/Game/Blueprints/Player/BaseCharacter.BaseCharacter_C")
        (set `self.AdvantageTip` false :!label _label_3)
        (goto _label_2)
        (elif (== _returnvalue "/Game/Blueprints/AI/BaseAI.BaseAI_C")
          (goto _label_3)
          (else
            (`self.StateFree`)))))))

(event `TipBall`
  ;[1 1 1 1 28] Tip Ball (Block or Rim)
  (`self.StateFree`)
  (if (`self.AdvantageTip`)
    (bind _outlaunchvelocity (`GameplayStatics.SuggestProjectileVelocity_CustomArc` (`self.K2_GetActorLocation` self) (`self.HoopTarget`) 0.0 (`self.AdvantageTipArc`)))
    (`PrimitiveComponent.SetPhysicsLinearVelocity` (`self.StaticMesh`) _outlaunchvelocity false "None")))

(event `StealBall`
  ;[1 1 1 1 28] Steal
  (`self.StateStolen`)
  (`PrimitiveComponent.SetPhysicsLinearVelocity` (`self.StaticMesh`) (`KismetMathLibrary.MakeVector` (`KismetMathLibrary.RandomFloatInRange` -250.0 250.0) (`KismetMathLibrary.RandomFloatInRange` -250.0 250.0) 250.0) false "None")
  (`self.K2_DetachFromActor` "KeepRelative"))

(event `StealCooldown`
  ;[1 1 1 1 28] Steal
  (`KismetSystemLibrary.Delay` 0.25)
  (`self.StateFree`))

(fn `UserConstructionScript`)