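; BaseCharacter is a character Blueprint with a follow camera that detects contact with balls for pickup.
; On any actor overlap, it gathers overlapping BaseBall actors and, if any exist, passes them to BallPickup on player 0's BaseCharacterController, whichever character overlapped.
; The construction script sets the camera's aspect ratio without constraining it and caches the skeletal mesh for socket use.
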(event `self.ReceiveActorBeginOverlap`
  (params (OtherActor :type "Actor Object Reference"))
  (bind _overlappingactors (`self.GetOverlappingActors` "/Game/Blueprints/BaseBall.BaseBall_C"))
  ;[1 1 1 1 28] Ball Overlap
  (if (!= (`KismetArrayLibrary.Array_Length` _overlappingactors) 0)
    (bind _asbase_character_controller (cast `/Game/Blueprints/BaseCharacterController` (`GameplayStatics.GetPlayerController` 0)))
    (`/Game/Blueprints/BaseCharacterController.BallPickup` _asbase_character_controller _overlappingactors)))

(fn `UserConstructionScript`
  (bind _followcamera (`self.FollowCamera`))
  ;[1 1 1 1 28] Camera Aspect Ratio
  (`CameraComponent.SetAspectRatio` _followcamera (`self.AspectRatio`))
  (`CameraComponent.SetConstraintAspectRatio` _followcamera false)
  ;[1 1 1 1 28] Skeletal Mesh Reference (for sockets)
  (set `self.PlayerSkeletalMesh` (`self.Mesh`)))