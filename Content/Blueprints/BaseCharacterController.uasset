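; Base character controller for a basketball game, handling movement and face-button combo input, with stubbed shoot, dribble and stun actions.
; Movement follows control yaw and is blocked while jumping.
; Face-button presses append digits to an ability string, which a delay started on first press clears; the started flag never resets.
; The completion check is never called, ability execution and shot meter are empty, and projectile-arc launch is unwired.
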(event `InputAxis|MoveForward`
  (params (AxisValue :type "Float (single-precision)"))
  ;[1 1 1 1 28] Move Input
  (if (not (`self.bIsJumping`))
    (`Pawn.AddMovementInput` (`GameplayStatics.GetPlayerCharacter` 0) (`KismetMathLibrary.GetForwardVector` (`KismetMathLibrary.MakeRotator` 0.0 0.0 (.yaw (`Pawn.GetControlRotation` (`GameplayStatics.GetPlayerCharacter` 0))))) AxisValue false)))

(event `InputAxis|MoveRight` :overrideparent false
  (params (AxisValue :type "Float (single-precision)"))
  ;[1 1 1 1 28] Move Input
  (if (not (`self.bIsJumping`))
    (`Pawn.AddMovementInput` (`GameplayStatics.GetPlayerCharacter` 0) (`KismetMathLibrary.GetRightVector` (`KismetMathLibrary.MakeRotator` 0.0 0.0 (.yaw (`Pawn.GetControlRotation` (`GameplayStatics.GetPlayerCharacter` 0))))) AxisValue false)))

(event `InputAction|FaceX`
  (params (Key :type "Key Structure"))
  ;[1 1 1 1 28] Ability Input
  (:`Pressed`
    (`/Engine/EditorBlueprintResources/StandardMacros.DoOnce` false :!label _label
      (:`Completed`
        (`self.CheckAbilityStart`)
        (set `self.AbilityString` (`KismetStringLibrary.Concat_StrStr` (`self.AbilityString`) "1")))))
  (:`Released`
    (goto _label :!via `Reset`)))

(event `InputAction|FaceSquare`
  (params (Key :type "Key Structure"))
  ;[1 1 1 1 28] Ability Input
  (:`Pressed`
    (`/Engine/EditorBlueprintResources/StandardMacros.DoOnce` false :!label _label_2
      (:`Completed`
        (`self.CheckAbilityStart`)
        (set `self.AbilityString` (`KismetStringLibrary.Concat_StrStr` (`self.AbilityString`) "2")))))
  (:`Released`
    (goto _label_2 :!via `Reset`)))

(event `InputAction|FaceCircle`
  (params (Key :type "Key Structure"))
  ;[1 1 1 1 28] Ability Input
  (:`Pressed`
    (`/Engine/EditorBlueprintResources/StandardMacros.DoOnce` false :!label _label_3
      (:`Completed`
        (`self.CheckAbilityStart`)
        (set `self.AbilityString` (`KismetStringLibrary.Concat_StrStr` (`self.AbilityString`) "3")))))
  (:`Released`
    (goto _label_3 :!via `Reset`)))

(event `InputAction|FaceTriangle`
  (params (Key :type "Key Structure"))
  ;[1 1 1 1 28] Ability Input
  (:`Pressed`
    (`/Engine/EditorBlueprintResources/StandardMacros.DoOnce` false :!label _label_4
      (:`Completed`
        (`self.CheckAbilityStart`)
        (set `self.AbilityString` (`KismetStringLibrary.Concat_StrStr` (`self.AbilityString`) "4")))))
  (:`Released`
    (goto _label_4 :!via `Reset`)))

(event `CheckAbilityStart`
  ;[1 1 1 1 28] Ability Input
  (if (not (`self.bAbilityStringStarted`))
    (set `self.bAbilityStringStarted` true)
    (`self.StartAbilityTimer`)))

(event `CheckAbilityCompletion`
  ;[1 1 1 1 28] Ability Input
  (if (>= (`KismetStringLibrary.Len` (`self.AbilityString`)) (`self.AbilityInputLength`))
    (`self.ExecuteAbility`)
    (set `self.AbilityString` "") ; Clear Ability String
  ))

(event `StartAbilityTimer`
  ;[1 1 1 1 28] Ability Input
  (`KismetSystemLibrary.Delay` (`self.AbilityTimerTime`))
  (set `self.AbilityString` "") ; Clear Ability String
)

(event `ExecuteAbility`
  ;[1 1 1 1 28] Ability Input
)

(event `Shoot`
  ;[1 1 1 1 28] Shoot
  (`self.StartShotMeter`) ; DOES NOTHING
)

(event `ShootResult`
  (params (ShootAttemptResult :type Integer))
  ;[1 1 1 1 28] Shoot
  (switch `int` ShootAttemptResult) ; 0 = Fail, 1 = Bounce, 2 = Swish
)

(event `Dribble`
  ;[1 1 1 1 28] Dribble
)

(event `StunMe`
  ;[1 1 1 1 28] Stun
)

(fn `StartShotMeter`)

(fn `UserConstructionScript`)