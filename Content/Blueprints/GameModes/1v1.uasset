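; 1v1 game mode Blueprint that keeps score between the player and an AI opponent.
; AddScore uses a selection index to add two points to either the player or the AI.
; UpdateScoreboard writes both totals as a dashed string to the Scoreboard's Score text, and AddScore calls it only when the player scores.
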(event `AddScore`
  (params (Selection :type Integer))
  ;[1 1 1 1 24] Score
  (switch `int` Selection
    (:`0`
      (set `self.PlayerScore` (+ (`self.PlayerScore`) 2))
      (`self.Update Scoreboard`))
    (:`1`
      (set `self.AIScore` (+ (`self.AIScore`) 2)))))

(event `Update Scoreboard`
  ;[1 1 1 1 24] Score
  (`TextBlock.SetText` (`/Game/UI/UMG_Scoreboard.Score` (`self.Scoreboard`)) (`KismetTextLibrary.Conv_StringToText` (`KismetStringLibrary.Concat_StrStr` (`KismetStringLibrary.Conv_IntToString` (`self.PlayerScore`)) " - " (`KismetStringLibrary.Conv_IntToString` (`self.AIScore`))))))

(fn `UserConstructionScript`)