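; Behavior Tree service that sets a basketball AI's phase and movement targets on the blackboard.
; Its first tick finds the first player, AI, hoop and ball, stores them as keys and caches both controllers and the ball.
; Later ticks select defense, offense or free-ball phase from possession and OffenseAI.
; Defense places the guard point GuardDistance from the player horizontally toward the hoop; free-ball targets the ball's location.
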(event `self.ReceiveTick`
  (params (OwnerActor :type "Actor Object Reference") (DeltaSeconds :type "Float (single-precision)"))
  (bind _returnvalue (`Actor.K2_GetActorLocation` (`BTFunctionLibrary.GetBlackboardValueAsActor` (`self.PlayerKey`))))
  (if (`self.bFirstTime`)
    (set `self.bFirstTime` false)
    ;[1 1 1] Set Player Key
    (bind _outactors (`GameplayStatics.GetAllActorsOfClass` "/Game/Blueprints/Player/BaseCharacter.BaseCharacter_C"))
    (bind _output (`|GetArrayItem` _outactors))
    (`BTFunctionLibrary.SetBlackboardValueAsObject` (`self.PlayerKey`) _output)
    (bind _returnvalue_2 (`Pawn.GetController` _output))
    (`BTFunctionLibrary.SetBlackboardValueAsObject` (`self.PlayerControllerKey`) _returnvalue_2)
    (bind _asbase_character_controller (cast `/Game/Blueprints/Player/BaseCharacterController` _returnvalue_2))
    (set `self.PlayerController` _asbase_character_controller)
    ;[1 1 1] Set AI Key
    (bind _outactors_2 (`GameplayStatics.GetAllActorsOfClass` "/Game/Blueprints/AI/BaseAI.BaseAI_C"))
    (bind _output_2 (`|GetArrayItem` _outactors_2))
    (`BTFunctionLibrary.SetBlackboardValueAsObject` (`self.AIKey`) _output_2)
    (bind _asbase_aicontroller (cast `/Game/Blueprints/AI/BaseAIController` (`AIBlueprintHelperLibrary.GetAIController` _output_2)))
    (set `self.AIController` _asbase_aicontroller)
    ;[1 1 1] Set Hoop Key
    (bind _outactors_3 (`GameplayStatics.GetAllActorsOfClass` "/Game/Blueprints/Hoop/BaseHoop.BaseHoop_C"))
    (`BTFunctionLibrary.SetBlackboardValueAsObject` (`self.HoopKey`) (`|GetArrayItem` _outactors_3))
    ;[1 1 1] Set Ball Key
    (bind _outactors_4 (`GameplayStatics.GetAllActorsOfClass` "/Game/Blueprints/Ball/BaseBall.BaseBall_C"))
    (bind _output_3 (`|GetArrayItem` _outactors_4))
    (`BTFunctionLibrary.SetBlackboardValueAsObject` (`self.BallKey`) _output_3)
    (bind _asbase_ball (cast `/Game/Blueprints/Ball/BaseBall` _output_3))
    (set `self.Ball` _asbase_ball)
    (elif (`/Game/Blueprints/Player/BaseCharacterController.bHasPossession` (`self.PlayerController`))
      (`BTFunctionLibrary.SetBlackboardValueAsInt` (`self.AiPhaseKey`) 1) ; Defense
      (`BTFunctionLibrary.SetBlackboardValueAsVector` (`self.GuardDestinationKey`) (+ _returnvalue (* (`KismetMathLibrary.GetDirectionUnitVector` (`KismetMathLibrary.MakeVector` (.x _returnvalue) (.y _returnvalue)) (`KismetMathLibrary.MakeVector` (.x (`Actor.K2_GetActorLocation` (`BTFunctionLibrary.GetBlackboardValueAsActor` (`self.HoopKey`)))) (.y (`Actor.K2_GetActorLocation` (`BTFunctionLibrary.GetBlackboardValueAsActor` (`self.HoopKey`)))))) (`self.GuardDistance`))))
      (elif (`/Game/Blueprints/AI/BaseAIController.bOffenseAI` (`self.AIController`))
        (`BTFunctionLibrary.SetBlackboardValueAsInt` (`self.AiPhaseKey`) 2) ; Offense
        (else
          (`BTFunctionLibrary.SetBlackboardValueAsInt` (`self.AiPhaseKey`)) ; Ball Free
          (`BTFunctionLibrary.SetBlackboardValueAsVector` (`self.BallChaseDestinationKey`) (`Actor.K2_GetActorLocation` (`self.Ball`))))))))