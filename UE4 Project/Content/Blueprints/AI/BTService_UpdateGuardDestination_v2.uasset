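; Behavior tree service that tracks ball possession and sets the basketball AI's phase and movement targets on the blackboard.
; Its first tick finds the player, AI, hoop and ball, fills their blackboard keys and caches the controllers and ball.
; Later ticks pick defense, offense or free ball from the controllers' possession state.
; Defense sets a guard point GuardDistance from the player toward the hoop, and a free ball sets the chase destination.
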(event `self.ReceiveTick`
  (params (OwnerActor :type "Actor Object Reference") (DeltaSeconds :type "Float (single-precision)"))
  (bind _returnvalue (`Actor.K2_GetActorLocation` (`BTFunctionLibrary.GetBlackboardValueAsActor` (`self.PlayerKey`))))
  (if (`self.bFirstTime`)
    (set `self.bFirstTime` false)
    ;[1 1 1] Set Player Key
    (bind _outactors (`GameplayStatics.GetAllActorsOfClass` "/Game/Blueprints/Player/BaseCharacter_v2.BaseCharacter_v2_C"))
    (bind _output (`|GetArrayItem` _outactors))
    (`BTFunctionLibrary.SetBlackboardValueAsObject` (`self.PlayerKey`) _output)
    (bind _returnvalue_2 (`Pawn.GetController` _output))
    (`BTFunctionLibrary.SetBlackboardValueAsObject` (`self.PlayerControllerKey`) _returnvalue_2)
    (bind _asbase_character_controller_v_2 (cast `/Game/Blueprints/Player/BaseCharacterController_v2` _returnvalue_2))
    (set `self.PlayerController` _asbase_character_controller_v_2)
    ;[1 1 1] Set AI Key
    (bind _outactors_2 (`GameplayStatics.GetAllActorsOfClass` "/Game/Blueprints/AI/BaseAI_v2.BaseAI_v2_C"))
    (bind _output_2 (`|GetArrayItem` _outactors_2))
    (`BTFunctionLibrary.SetBlackboardValueAsObject` (`self.AIKey`) _output_2)
    (bind _asbase_aicontroller_v_2 (cast `/Game/Blueprints/AI/BaseAIController_v2` (`AIBlueprintHelperLibrary.GetAIController` _output_2)))
    (set `self.AIController` _asbase_aicontroller_v_2)
    ;[1 1 1] Set Hoop Key
    (bind _outactors_3 (`GameplayStatics.GetAllActorsOfClass` "/Game/Blueprints/Hoop/BaseHoop_v2.BaseHoop_v2_C"))
    (`BTFunctionLibrary.SetBlackboardValueAsObject` (`self.HoopKey`) (`|GetArrayItem` _outactors_3))
    ;[1 1 1] Set Ball Key
    (bind _outactors_4 (`GameplayStatics.GetAllActorsOfClass` "/Game/Blueprints/Ball/BaseBall_v2.BaseBall_v2_C"))
    (bind _output_3 (`|GetArrayItem` _outactors_4))
    (`BTFunctionLibrary.SetBlackboardValueAsObject` (`self.BallKey`) _output_3)
    (set `self.Ball` _output_3)
    (elif (`/Game/Blueprints/Player/BaseCharacterController_v2.bHasPossession` (`self.PlayerController`))
      (`BTFunctionLibrary.SetBlackboardValueAsInt` (`self.AiPhaseKey`) 1) ; Defense
      (`BTFunctionLibrary.SetBlackboardValueAsVector` (`self.GuardDestinationKey`) (+ _returnvalue (* (`KismetMathLibrary.GetDirectionUnitVector` (`KismetMathLibrary.MakeVector` (.x _returnvalue) (.y _returnvalue)) (`KismetMathLibrary.MakeVector` (.x (`Actor.K2_GetActorLocation` (`BTFunctionLibrary.GetBlackboardValueAsActor` (`self.HoopKey`)))) (.y (`Actor.K2_GetActorLocation` (`BTFunctionLibrary.GetBlackboardValueAsActor` (`self.HoopKey`)))))) (`self.GuardDistance`))))
      (elif (`/Game/Blueprints/AI/BaseAIController_v2.bOffenseAI` (`self.AIController`))
        (`BTFunctionLibrary.SetBlackboardValueAsInt` (`self.AiPhaseKey`) 2) ; Offense
        (else
          (`BTFunctionLibrary.SetBlackboardValueAsInt` (`self.AiPhaseKey`)) ; Ball Free
          (`BTFunctionLibrary.SetBlackboardValueAsVector` (`self.BallChaseDestinationKey`) (`Actor.K2_GetActorLocation` (`self.Ball`))))))))