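; AI controller for a basketball opponent that steals, blocks shots, gets stunned or countered, and handles ball pickup by offense or defense role.
; BeginPlay caches the ball, player, hoop and pawn detectors, then runs a behavior tree.
; Blackboard bools gate stun, steal and block, with randomized cooldowns re-enabling the latter two.
; Blocks launch the pawn along the ball-to-hoop direction; play resets teleport it by role, optionally switching sides.
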(event `self.ReceiveBeginPlay`
  ;[1 1 1 1 28] Begin Play
  (`self.DefineTheBall`)
  (`self.DefineThePlayer`)
  (`self.DefineMyAIMySkeleton`)
  (`self.DefineTheHoop`)
  (`self.RunBehaviorTree` (`self.BehaviorTree`))
  (`self.StealCooldown`)
  (`self.BlockCooldown`))

(event `DefineTheBall`
  ;[1 1 1 1 28] Begin Play
  (bind _outactors (`GameplayStatics.GetAllActorsOfClass` "/Game/Blueprints/Ball/BaseBall_v1.BaseBall_v1_C"))
  (set `self.TheBall` (`|GetArrayItem` _outactors)))

(event `DefineThePlayer`
  ;[1 1 1 1 28] Begin Play
  (bind _outactors (`GameplayStatics.GetAllActorsOfClass` "/Game/Blueprints/Player/BaseCharacter_v2.BaseCharacter_v2_C"))
  (bind _output_get (set `self.ThePlayer` (`|GetArrayItem` _outactors)))
  (set `self.PlayerStunDetector` (`/Game/Blueprints/Player/BaseCharacter_v2.StunDetector` _output_get)))

(event `DefineMyAIMySkeleton`
  ;[1 1 1 1 28] Begin Play
  (bind _asbase_ai (cast `/Game/Blueprints/AI/BaseAI` (`self.K2_GetPawn`)))
  (bind _output_get (set `self.MyAiCharacter` _asbase_ai))
  (set `self.MySkeletalMesh` (`/Game/Blueprints/AI/BaseAI.AISkeletalMesh` _output_get))
  (set `self.MyStunDetector` (`/Game/Blueprints/AI/BaseAI.StunDetector` (`self.MyAiCharacter`)))
  (set `self.MyBlockDetector` (`/Game/Blueprints/AI/BaseAI.BlockDetector` (`self.MyAiCharacter`))))

(event `DefineTheHoop`
  ;[1 1 1 1 28] Begin Play
  (bind _outactors (`GameplayStatics.GetAllActorsOfClass` "/Game/Blueprints/Hoop/BaseHoop.BaseHoop_C"))
  (bind _output_get (set `self.TheHoop` (`|GetArrayItem` _outactors)))
  (set `self.HoopTarget` (`self.K2_GetActorLocation` _output_get)))

(event `StunMe`
  (params (StunDelay :type "Float (double-precision)"))
  ;[1 1 1 1 28] Stun/Counter Me
  (`/Game/Blueprints/AI/BaseAI.SetMaterialStunned` (`self.MyAiCharacter`))
  (`BlackboardComponent.SetValueAsBool` (`AIBlueprintHelperLibrary.GetBlackboard` self) (`self.StunKey`) true)
  (`KismetSystemLibrary.Delay` StunDelay)
  (`KismetSystemLibrary.PrintString` "AI no longer stunned" :!label _label)
  (`BlackboardComponent.SetValueAsBool` (`AIBlueprintHelperLibrary.GetBlackboard` self) (`self.StunKey`) false)
  (`/Game/Blueprints/AI/BaseAI.SetMaterialNormal` (`self.MyAiCharacter`)))

(event `CounterMe`
  (params (StunDelay :type "Float (double-precision)"))
  ;[1 1 1 1 28] Stun/Counter Me
  (`/Game/Blueprints/AI/BaseAI.SetMaterialCountered` (`self.MyAiCharacter`))
  (`BlackboardComponent.SetValueAsBool` (`AIBlueprintHelperLibrary.GetBlackboard` self) (`self.StunKey`) true)
  (`KismetSystemLibrary.Delay` StunDelay)
  (goto _label))

(event `Steal`
  (bind _overlappingactors (`PrimitiveComponent.GetOverlappingActors` (`self.MyStunDetector`) "/Game/Blueprints/Player/BaseCharacter.BaseCharacter_C"))
  ;[1 1 1 1 28] Steal
  (if (`BlackboardComponent.GetValueAsBool` (`AIBlueprintHelperLibrary.GetBlackboard` self) (`self.StealKey`))
    (if (> (`KismetArrayLibrary.Array_Length` _overlappingactors) 0)
      (bind _asbase_character (cast `/Game/Blueprints/Player/BaseCharacter` (`|GetArrayItem` _overlappingactors)))
      (bind _asbase_character_controller_v_2 (cast `/Game/Blueprints/Player/BaseCharacterController_v2` (`Pawn.GetController` _asbase_character)))
      (if (`/Game/Blueprints/Player/BaseCharacterController_v2.bHasPossession` _asbase_character_controller_v_2)
        (`self.SetCanSteal` false)
        (set `self.bIsStealing` true)
        (`/Game/Blueprints/Player/BaseCharacterController_v2.PlayerStealFromMe` _asbase_character_controller_v_2 self)
        (`self.StealCooldown`)
        (`/Game/Blueprints/AI/BaseAI.SetMaterialStealing` (`self.MyAiCharacter`))))))

(event `SetCanSteal`
  (params (BoolValue :type Boolean))
  ;[1 1 1 1 28] Steal
  (`BlackboardComponent.SetValueAsBool` (`AIBlueprintHelperLibrary.GetBlackboard` self) (`self.StealKey`) BoolValue))

(event `StealCooldown`
  ;[1 1 1 1 28] Steal
  (`KismetSystemLibrary.Delay` 0.1)
  (set `self.bIsStealing` false)
  (`KismetSystemLibrary.Delay` (`KismetMathLibrary.RandomFloatInRange` (`self.StealCooldownTimeMin`) (`self.StealCooldownTimeMax`)))
  (`self.SetCanSteal` true))

(event `AIStealFromMe`
  ;[1 1 1] Steal From Me
  (`KismetSystemLibrary.PrintString` "AI STOLEN")
  (`/Game/Blueprints/Ball/BaseBall_v1.StealBall` (`self.TheBall`))
  (set `self.bHasPossession` false))

(event `BlockAttempt`
  (bind _overlappingactors (`PrimitiveComponent.GetOverlappingActors` (`self.MyBlockDetector`) "/Game/Blueprints/Player/BaseCharacter.BaseCharacter_C"))
  ;[1 1 1 1 28] Block
  (if (`BlackboardComponent.GetValueAsBool` (`AIBlueprintHelperLibrary.GetBlackboard` self) (`self.BlockKey`))
    (if (> (`KismetArrayLibrary.Array_Length` _overlappingactors) 0)
      (bind _asbase_character (cast `/Game/Blueprints/Player/BaseCharacter` (`|GetArrayItem` _overlappingactors)))
      (bind _asbase_character_controller (cast `/Game/Blueprints/Player/BaseCharacterController` (`Pawn.GetController` _asbase_character)))
      (if (`/Game/Blueprints/Player/BaseCharacterController.bHasPossession` _asbase_character_controller)
        (if (`/Game/Blueprints/Player/BaseCharacterController.bShotActive` _asbase_character_controller)
          (`/Engine/EditorBlueprintResources/StandardMacros.DoOnce` false :!label _label_2
            (:`Completed`
              (`self.SetCanBlock` false)
              (`self.BlockCooldown`)
              (`self.Block`)))
          (else
            (goto _label_2 :!via `Reset`)))))))

(event `Block`
  ;[1 1 1 1 28] Block
  (`KismetSystemLibrary.PrintString` "Blocking")
  (`self.BlockVector`))

(event `SetCanBlock`
  (params (`Bool Value` :type Boolean))
  ;[1 1 1 1 28] Block
  (`BlackboardComponent.SetValueAsBool` (`AIBlueprintHelperLibrary.GetBlackboard` self) (`self.BlockKey`) `Bool Value`))

(event `BlockVector`
  ;[1 1 1 1 28] Block
  (`self.BlockJump` (* (`KismetMathLibrary.GetDirectionUnitVector` (`self.K2_GetActorLocation` (`self.TheBall`)) (`self.K2_GetActorLocation` (`self.TheHoop`))) 10.0)))

(event `BlockJump`
  (params (LaunchVelocity :type "Vector Structure"))
  ;[1 1 1 1 28] Block
  (`Character.LaunchCharacter` (`self.MyAiCharacter`) (* LaunchVelocity (`self.BlockFactor`)) false false))

(event `BlockCooldown`
  ;[1 1 1 1 28] Block
  (`KismetSystemLibrary.Delay` (`KismetMathLibrary.RandomFloatInRange` (`self.BlockCooldownTimeMin`) (`self.BlockCooldownTimeMax`)))
  (`self.SetCanBlock` true))

(event `AIBallPickup`
  (params (Ball :type "/Game/Blueprints/Ball/BaseBall_v1 Object Reference"))
  ;[1 1 1 1 24] Ball Pickup
  (if (`self.bOffenseAI`)
    (`self.OffenseBallCheck` Ball)
    (else
      (`self.DefenseBallCheck` Ball))))

(event `DefenseBallCheck`
  (params (Ball :type "/Game/Blueprints/Ball/BaseBall_v1 Object Reference"))
  ;[1 1 1 1 24] Ball Pickup
  (if (`/Game/Blueprints/Ball/BaseBall_v1.bIsShot` Ball)
    (`KismetSystemLibrary.PrintString` "can't pickup ball")
    (else
      (set `/Game/Blueprints/Ball/BaseBall_v1.bPossessable` false Ball)
      (`BlackboardComponent.SetValueAsBool` (`AIBlueprintHelperLibrary.GetBlackboard` self) (`KismetStringLibrary.Conv_StringToName` "bSwitchSides") true))))

(event `OffenseBallCheck`
  (params (Ball :type "/Game/Blueprints/Ball/BaseBall_v1 Object Reference"))
  ;[1 1 1 1 24] Ball Pickup
  (if (`/Game/Blueprints/Ball/BaseBall_v1.bPossessable` Ball)
    (`/Game/Blueprints/Ball/BaseBall_v1.PickUpBall` (`self.TheBall`) (`self.MySkeletalMesh`) (`self.BallRHandSocket`))
    (set `self.bHasPossession` true)))

(event `ResetPlayAIPlayer`
  (params (OffensePosition :type "Vector Structure") (DefensePosition :type "Vector Structure") (SwitchSides :type Boolean))
  (bind _myaicharacter (`self.MyAiCharacter`))
  (bind _myaicharacter_2 (`self.MyAiCharacter`))
  ;[1 1 1 1 24] Reset Play
  (if SwitchSides
    (set `self.bOffenseAI` (not (`self.bOffenseAI`))))
  (if (`self.bOffenseAI`)
    (`MovementComponent.StopMovementImmediately` (`Pawn.GetMovementComponent` _myaicharacter))
    (`self.K2_TeleportTo` :`self` _myaicharacter :`DestLocation` OffensePosition)
    (else
      (`MovementComponent.StopMovementImmediately` (`Pawn.GetMovementComponent` _myaicharacter_2))
      (`self.K2_TeleportTo` :`self` _myaicharacter_2 :`DestLocation` DefensePosition))))

(fn `UserConstructionScript`)