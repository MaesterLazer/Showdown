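; Basketball actor that handles pickup, shooting, stealing, tipping and resets to a spawn found at BeginPlay.
; State events swap collision profiles, physics and possessability, with swish shots skipping hoop collision.
; Mid-shot hits free the ball, and advantage shots hitting the rim relaunch toward the hoop on a computed arc.
; Steals pop it randomly sideways until a cooldown frees it, and out-of-bounds overlaps trigger the 1v1 game mode's reset.
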(event `self.ReceiveBeginPlay`
  ;[1 1 1 1 28] Startup
  (`|ExecutionSequence`
    (:`then_0`
      (`self.DefineTheHoopTarget`))
    (:`then_1`
      (`self.DefineBallSpawn`))))

(event `DefineTheHoopTarget`
  ;[1 1 1 1 28] Startup
  (bind _outactors (`GameplayStatics.GetAllActorsOfClass` "/Game/Blueprints/Hoop/BaseHoop.BaseHoop_C"))
  (set `self.HoopTarget` (`self.K2_GetActorLocation` (`|GetArrayItem` _outactors)))
  (bind _returnvalue (`KismetArrayLibrary.Array_Length` _outactors))
  (if (!= _returnvalue 0)
    (if (> _returnvalue 1)
      (`KismetSystemLibrary.PrintString` "More than 1 hoop in scene." false))
    (else
      (`KismetSystemLibrary.PrintString` "No hoops in scene." false))))

(event `DefineBallSpawn`
  ;[1 1 1 1 28] Startup
  (bind _outactors (`GameplayStatics.GetAllActorsOfClass` "/Game/Blueprints/Ball/DEPRECATE_bp_BallSpawn.DEPRECATE_bp_BallSpawn_C"))
  (bind _asdeprecate_bp_ball_spawn (cast `/Game/Blueprints/Ball/DEPRECATE_bp_BallSpawn` (`|GetArrayItem` _outactors)))
  (set `self.BallSpawn` _asdeprecate_bp_ball_spawn)
  (bind _returnvalue (`KismetArrayLibrary.Array_Length` _outactors))
  (if (!= _returnvalue 0)
    (if (> _returnvalue 1)
      (`KismetSystemLibrary.PrintString` "More than 1 ball spawn in scene." false))
    (else
      (`KismetSystemLibrary.PrintString` "No ball sspawn in scene." false))))

(event `ResetPlayBall`
  ;[1 1 1 1 28] ResetPlay
  (`self.K2_DetachFromActor` "KeepRelative")
  (`self.StateFree`)
  (`PrimitiveComponent.SetPhysicsLinearVelocity` (`self.StaticMesh`) (0.0 0.0 0.0) false "None")
  (`self.K2_TeleportTo` (`self.K2_GetActorLocation` (`self.BallSpawn`)))
  (set `self.bIsShot` false)
  (set `self.bPossessable` true))

(event `StateFree`
  ;[1 1 1 1 28] States
  (`PrimitiveComponent.SetCollisionProfileName` (`self.StaticMesh`) "BallFree" true)
  (`PrimitiveComponent.SetSimulatePhysics` (`self.StaticMesh`) true)
  (set `PrimitiveComponent.bGenerateOverlapEvents` true (`self.StaticMesh`))
  (set `self.bPossessable` true)
  (set `self.bIsShot` false)
  (set `self.DebugBallState` "Free"))

(event `StatePossessed`
  ;[1 1 1 1 28] States
  (`PrimitiveComponent.SetSimulatePhysics` (`self.StaticMesh`) false)
  (`PrimitiveComponent.SetCollisionProfileName` (`self.StaticMesh`) "BallPossessed" true)
  (set `self.bPossessable` false)
  (set `self.DebugBallState` "Posessed"))

(event `StateShot`
  ;[1 1 1 1 28] States
  (`PrimitiveComponent.SetCollisionProfileName` (`self.StaticMesh`) "BallFree" true)
  (`PrimitiveComponent.SetSimulatePhysics` (`self.StaticMesh`) true)
  (set `PrimitiveComponent.bGenerateOverlapEvents` false (`self.StaticMesh`)) ; Might not be necessary
  (set `self.bPossessable` false)
  (set `self.DebugBallState` "Shot"))

(event `StateStolen`
  ;[1 1 1 1 28] States
  (`PrimitiveComponent.SetCollisionProfileName` (`self.StaticMesh`) "BallStolen" true)
  (`PrimitiveComponent.SetSimulatePhysics` (`self.StaticMesh`) true)
  (set `PrimitiveComponent.bGenerateOverlapEvents` true (`self.StaticMesh`))
  (set `self.bPossessable` false)
  (set `self.DebugBallState` "Stolen")
  (`self.StealCooldown`))

(event `StateSwish`
  ;[1 1 1 1 28] States
  (`PrimitiveComponent.SetCollisionProfileName` (`self.StaticMesh`) "BallSwish" true)
  (`PrimitiveComponent.SetSimulatePhysics` (`self.StaticMesh`) true)
  (set `self.bPossessable` false)
  (set `self.DebugBallState` "Swish"))

(event `StateReset`
  ;[1 1 1 1 28] States
  (`PrimitiveComponent.SetCollisionProfileName` (`self.StaticMesh`) "BallFree" true)
  (`PrimitiveComponent.SetSimulatePhysics` (`self.StaticMesh`) true)
  (set `self.DebugBallState` "Reset"))

(event `AttachBallTo`
  (params (Parent :type "SceneComponent Object Reference") (SocketName :type Name))
  ;[1 1 1 1 28] Attach
  (`self.K2_AttachToComponent` Parent SocketName "SnapToTarget" "KeepRelative" "KeepRelative" false))

(event `PickUpBall`
  (params (Parent :type "SceneComponent Object Reference") (SocketName :type Name))
  ;[1 1 1 1 28] Pick Up
  (if (`self.bPossessable`)
    (`self.StatePossessed`)
    (`self.AttachBallTo` Parent SocketName)))

(event `ShootBall`
  (params (LaunchVelocity :type "Vector Structure") (Selection :type Integer))
  ;[1 1 1 1 28] Shoot
  (switch `int` Selection
    (:`0`
      (set `self.bAdvantageTip` false)
      (`self.StateShot` :!label _label))
    (:`1`
      (set `self.bAdvantageTip` true)
      (goto _label))
    (:`2`
      (`self.StateSwish`)))
  (`PrimitiveComponent.SetPhysicsLinearVelocity` (`self.StaticMesh`) LaunchVelocity false "None")
  (`self.K2_DetachFromActor` "KeepRelative")
  (set `self.bIsShot` true))

(event `self.StaticMesh.OnComponentHit`
  (params (HitComponent :type "PrimitiveComponent Object Reference") (OtherActor :type "Actor Object Reference") (OtherComp :type "PrimitiveComponent Object Reference") (NormalImpulse :type "Vector Structure") (Hit :type "HitResult Structure (by ref)"))
  (bind _returnvalue (`GameplayStatics.GetObjectClass` OtherActor))
  ;[1 1 1 1 28] Mid-Shot Collision (Hoop/Person/Other)
  (if (`self.bPossessable`)
    _
    (elif (`self.bIsShot`)
      (if (== _returnvalue "/Game/Blueprints/Hoop/BaseHoop.BaseHoop_C")
        (`self.TipBall`)
        (else
          (if (== _returnvalue "/Game/Blueprints/Player/BaseCharacter.BaseCharacter_C")
            (set `self.bAdvantageTip` false :!label _label_2)
            (`self.TipBall`)
            (elif (== _returnvalue "/Game/Blueprints/AI/BaseAI.BaseAI_C")
              (goto _label_2)
              (else
                (`self.StateFree`))))
          (set `self.bIsShot` false)
          (set `self.bPossessable` true)
          ;[1 1 1 1 28] Tip Ball (Block or Rim)
          (`KismetSystemLibrary.PrintString` "Ball is possessable" :!label _label_3))))))

(event `TipBall`
  ;[1 1 1 1 28] Tip Ball (Block or Rim)
  (`self.StateFree`)
  (if (`self.bAdvantageTip`)
    (bind _outlaunchvelocity (`GameplayStatics.SuggestProjectileVelocity_CustomArc` (`self.K2_GetActorLocation` self) (`self.HoopTarget`) 0.0 (`self.AdvantageTipArc`)))
    (`PrimitiveComponent.SetPhysicsLinearVelocity` (`self.StaticMesh`) _outlaunchvelocity false "None"))
  (set `self.bIsShot` false)
  (set `self.bPossessable` true)
  (goto _label_3))

(event `StealBall`
  ;[1 1 1 1 28] Steal
  (`self.StateStolen`)
  (`PrimitiveComponent.SetPhysicsLinearVelocity` (`self.StaticMesh`) (`KismetMathLibrary.MakeVector` (* (`KismetMathLibrary.RandomFloatInRange` (`self.StealPowerMin`) (`self.StealPowerMax`)) (- (* (`KismetMathLibrary.RandomIntegerInRange` 0 1) 2.0) 1.0)) 0.0 250.0) false "None")
  (`self.K2_DetachFromActor` "KeepRelative"))

(event `StealCooldown`
  ;[1 1 1 1 28] Steal
  (`KismetSystemLibrary.Delay` (`self.StolenCooldown`))
  (`self.StateFree`))

(event `self.StaticMesh.OnComponentBeginOverlap`
  (params (OverlappedComponent :type "PrimitiveComponent Object Reference") (OtherActor :type "Actor Object Reference") (OtherComp :type "PrimitiveComponent Object Reference") (OtherBodyIndex :type Integer) (bFromSweep :type Boolean) (SweepResult :type "HitResult Structure (by ref)"))
  ;[1 1 1 1 28] OutOfBounds
  (if (`self.ActorHasTag` OtherActor (`self.OutOfBoundsTag`))
    (bind _as1v_1_game_mode (cast `/Game/Blueprints/GameModes/1v1_GameMode` (`GameplayStatics.GetGameMode`))) ; CLEAN UP
    (`/Game/Blueprints/GameModes/1v1_GameMode.ResetPlayGamemode` _as1v_1_game_mode 2) ; ResetType: 0 = Shotclock, 1 = Score, 2 = Out of Bounds
  ))

(fn `UserConstructionScript`)