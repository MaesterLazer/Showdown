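; Basketball actor for a 1v1 game, handling pickup, shooting, steals, tips and resets.
; State events swap collision profiles, physics and possession eligibility, then notify the GameState as Free or Possessed.
; Shots detach and launch the ball; hoop or character hits tip it free, with advantage rim tips re-arced toward the hoop via SuggestProjectileVelocityCustomArc.
; Steals pop it randomly sideways until a cooldown frees it; out-of-bounds overlaps call GameMode's DetermineSides.
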(event `ShowdownInterface.EventOnRegisterGameObjects`
  (params (newGameObjects :type "GameplayObjects Structure"))
  (set `self.SpawnPos` (`.BallStartPos` (break `GameplayObjects` newGameObjects)))
  (set `self.HoopTarget` (`self.K2_GetActorLocation` (`.Hoop` (break `GameplayObjects` newGameObjects))))
  (set `self.bPossessable` true))

(event `ResetPlayBall`
  ;[1 1 1 1 28] ResetPlay
  (`self.K2_DetachFromActor` "KeepRelative")
  (`self.StateFree`)
  (`PrimitiveComponent.SetPhysicsLinearVelocity` (`self.StaticMesh`) (0.0 0.0 0.0) false "None")
  (`self.K2_SetActorLocation` (`self.SpawnPos`) false true)
  (set `self.bIsShot` false)
  (set `self.bPossessable` true))

(event `StateFree`
  ;[1 1 1 1 28] States
  (`PrimitiveComponent.SetCollisionProfileName` (`self.StaticMesh`) "BallFree" true)
  (`PrimitiveComponent.SetSimulatePhysics` (`self.StaticMesh`) true)
  (set `PrimitiveComponent.bGenerateOverlapEvents` true (`self.StaticMesh`))
  (set `self.bPossessable` true)
  (set `self.bIsShot` false)
  (set `self.DebugBallState` "Free")
  (message `ShowdownInterface.EventBallStateChange` (`GameplayStatics.GetGameState`) "Free"))

(event `StatePossessed`
  ;[1 1 1 1 28] States
  (`PrimitiveComponent.SetSimulatePhysics` (`self.StaticMesh`) false)
  (`PrimitiveComponent.SetCollisionProfileName` (`self.StaticMesh`) "BallPossessed" true)
  (set `self.bPossessable` false)
  (set `self.DebugBallState` "Posessed")
  (message `ShowdownInterface.EventBallStateChange` (`GameplayStatics.GetGameState`) "Possessed"))

(event `StateShot`
  ;[1 1 1 1 28] States
  (`PrimitiveComponent.SetCollisionProfileName` (`self.StaticMesh`) "BallFree" true)
  (`PrimitiveComponent.SetSimulatePhysics` (`self.StaticMesh`) true)
  (set `PrimitiveComponent.bGenerateOverlapEvents` false (`self.StaticMesh`)) ; Might not be necessary
  (set `self.bPossessable` false)
  (set `self.DebugBallState` "Shot")
  (message `ShowdownInterface.EventBallStateChange` (`GameplayStatics.GetGameState`) "Free" :!label _label))

(event `StateStolen`
  ;[1 1 1 1 28] States
  (`PrimitiveComponent.SetCollisionProfileName` (`self.StaticMesh`) "BallStolen" true)
  (`PrimitiveComponent.SetSimulatePhysics` (`self.StaticMesh`) true)
  (set `PrimitiveComponent.bGenerateOverlapEvents` true (`self.StaticMesh`))
  (set `self.bPossessable` false)
  (set `self.DebugBallState` "Stolen")
  (`self.StealCooldown`)
  (goto _label))

(event `StateSwish`
  ;[1 1 1 1 28] States
  (`PrimitiveComponent.SetCollisionProfileName` (`self.StaticMesh`) "BallSwish" true)
  (`PrimitiveComponent.SetSimulatePhysics` (`self.StaticMesh`) true)
  (set `self.bPossessable` false)
  (set `self.DebugBallState` "Swish")
  (message `ShowdownInterface.EventBallStateChange` (`GameplayStatics.GetGameState`) "Free" :!label _label_2))

(event `StateReset`
  ;[1 1 1 1 28] States
  (`PrimitiveComponent.SetCollisionProfileName` (`self.StaticMesh`) "BallFree" true)
  (`PrimitiveComponent.SetSimulatePhysics` (`self.StaticMesh`) true)
  (set `self.DebugBallState` "Reset")
  (goto _label_2))

(event `AttachBallTo`
  (params (Parent :type "SceneComponent Object Reference") (SocketName :type Name))
  ;[1 1 1 1 28] Attach
  (`self.K2_AttachToComponent` Parent SocketName "SnapToTarget" "KeepRelative" "KeepRelative" false))

(event `PickUpBall`
  (params (Parent :type "SceneComponent Object Reference") (SocketName :type Name))
  ;[1 1 1 1 28] Pick Up
  (if (`self.bPossessable`)
    (`self.StatePossessed`)
    (`self.AttachBallTo` Parent SocketName)))

(event `ShootBall`
  (params (LaunchVelocity :type "Vector Structure") (Selection :type Integer))
  ;[1 1 1 1 28] Shoot
  (switch `int` Selection
    (:`0`
      (set `self.bAdvantageTip` false)
      (`self.StateShot` :!label _label_3))
    (:`1`
      (set `self.bAdvantageTip` true)
      (goto _label_3))
    (:`2`
      (`self.StateSwish`)))
  (`PrimitiveComponent.SetPhysicsLinearVelocity` (`self.StaticMesh`) LaunchVelocity false "None")
  (`self.K2_DetachFromActor` "KeepRelative")
  (set `self.bIsShot` true))

(event `self.StaticMesh.OnComponentHit`
  (params (HitComponent :type "PrimitiveComponent Object Reference") (OtherActor :type "Actor Object Reference") (OtherComp :type "PrimitiveComponent Object Reference") (NormalImpulse :type "Vector Structure") (Hit :type "HitResult Structure (by ref)"))
  (bind _returnvalue (`GameplayStatics.GetObjectClass` OtherActor))
  ;[1 1 1 1 28] Mid-Shot Collision (Hoop/Person/Other)
  (if (`self.bPossessable`)
    _
    (elif (`self.bIsShot`)
      (if (== _returnvalue "/Game/Blueprints/Hoop/BaseHoop.BaseHoop_C")
        (`self.TipBall`)
        (else
          (if (== _returnvalue "/Game/Blueprints/Player/BaseCharacterController.BaseCharacterController_C")
            (set `self.bAdvantageTip` false :!label _label_4)
            (`self.TipBall`)
            (elif (== _returnvalue "/Game/Blueprints/AI/BaseAI.BaseAI_C")
              (goto _label_4)
              (else
                (`self.StateFree`))))
          (set `self.bIsShot` false)
          (set `self.bPossessable` true)
          ;[1 1 1 1 28] Tip Ball (Block or Rim)
          (`KismetSystemLibrary.PrintString` "Ball is possessable" :!label _label_5))))))

(event `TipBall`
  ;[1 1 1 1 28] Tip Ball (Block or Rim)
  (`self.StateFree`)
  (if (`self.bAdvantageTip`)
    (bind _outlaunchvelocity (`GameplayStatics.SuggestProjectileVelocity_CustomArc` (`self.K2_GetActorLocation` self) (`self.HoopTarget`) 0.0 (`self.AdvantageTipArc`)))
    (`PrimitiveComponent.SetPhysicsLinearVelocity` (`self.StaticMesh`) _outlaunchvelocity false "None"))
  (set `self.bIsShot` false)
  (set `self.bPossessable` true)
  (goto _label_5))

(event `StealBall`
  ;[1 1 1 1 28] Steal
  (`self.StateStolen`)
  (`PrimitiveComponent.SetPhysicsLinearVelocity` (`self.StaticMesh`) (`KismetMathLibrary.MakeVector` (* (`KismetMathLibrary.RandomFloatInRange` (`self.StealPowerMin`) (`self.StealPowerMax`)) (- (* (`KismetMathLibrary.RandomIntegerInRange` 0 1) 2.0) 1.0)) 0.0 250.0) false "None")
  (`self.K2_DetachFromActor` "KeepRelative"))

(event `StealCooldown`
  ;[1 1 1 1 28] Steal
  (`KismetSystemLibrary.Delay` (`self.StolenCooldown`))
  (`self.StateFree`))

(event `self.StaticMesh.OnComponentBeginOverlap`
  (params (OverlappedComponent :type "PrimitiveComponent Object Reference") (OtherActor :type "Actor Object Reference") (OtherComp :type "PrimitiveComponent Object Reference") (OtherBodyIndex :type Integer) (bFromSweep :type Boolean) (SweepResult :type "HitResult Structure (by ref)"))
  ;[1 1 1 1 28] OutOfBounds
  (if (`self.ActorHasTag` OtherActor (`self.OutOfBoundsTag`))
    (`/Game/Blueprints/GameModes/1v1_GameMode.DetermineSides` (cast `/Game/Blueprints/GameModes/1v1_GameMode` (`GameplayStatics.GetGameMode`) :!pure true) "OutOfBounds")))

(fn `UserConstructionScript`)