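; 1v1 basketball game mode that runs scoring, game clock and shot clock for a player-versus-AI match.
; Looping one-second timers update the scoreboard clocks, and a shot clock expiry shows a violation popup.
; Scores, violations and other reset types route through DetermineSides, which sets side switching and shot clock reset, then resets player, AI and ball.
; Only the player's score branch calls the scoreboard update and post-score reset.
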(event `self.ReceiveBeginPlay`
  ;[1 1 1 1 24] Begin Play
  (`self.Start Gameclock`))

(event `GetStartingPositions`
  ;[1 1 1 1 24] Begin Play
  (set `self.OffenseStartingPosition` (`self.K2_GetActorLocation` (`self.K2_FindPlayerStart` (`self.Player`))))
  (set `self.DefenseStartingPosition` (`self.K2_GetActorLocation` (`/Game/Blueprints/AI/BaseAIController.MyAiCharacter` (`self.AI`)))))

(event `AddScore`
  (params (Selection :type Integer))
  ;[1 1 1 1 24] Score
  (switch `int` Selection
    (:`0`
      (set `self.PlayerScore` (+ (`self.PlayerScore`) 2))
      (`self.Update Scoreboard`))
    (:`1`
      (set `self.AIScore` (+ (`self.AIScore`) 2)))))

(event `Update Scoreboard`
  ;[1 1 1 1 24] Score
  (`TextBlock.SetText` (`/Game/UI/UMG_Scoreboard.Score` (`self.Scoreboard`)) (`KismetTextLibrary.Conv_StringToText` (`KismetStringLibrary.Concat_StrStr` (`KismetStringLibrary.Conv_IntToString` (`self.PlayerScore`)) " - " (`KismetStringLibrary.Conv_IntToString` (`self.AIScore`)))))
  (`KismetSystemLibrary.Delay` 1.0)
  (`self.ResetPlayGamemode` 1) ; ResetType: 0 = Shotclock, 1 = Score
)

(event `Start Gameclock`
  ;[1 1 1 1 24] Score
  (`KismetSystemLibrary.Delay` 1.0)
  (`TextBlock.SetText` (`/Game/UI/UMG_Scoreboard.Gametime` (`self.Scoreboard`)) (`KismetTextLibrary.Conv_StringToText` (`KismetStringLibrary.Concat_StrStr` "1" ":" "00")))
  (set `self.GameTime` 0)
  (`KismetSystemLibrary.K2_SetTimerDelegate` (delegate `Update Gameclock`) 1.0 true)
  (set `self.ShotClockTime` 0)
  (`KismetSystemLibrary.K2_SetTimerDelegate` (delegate `UpdateShotClock`) 1.0 true))

(event `Update Gameclock`
  (bind (_remainder _returnvalue) (`KismetMathLibrary.FMod` (`KismetMathLibrary.Conv_IntToDouble` (- (`self.GameTimeLimit`) (`self.GameTime`))) 60.0))
  ;[1 1 1 1 24] Score
  (set `self.GameTime` (+ (`self.GameTime`) 1))
  (`TextBlock.SetText` (`/Game/UI/UMG_Scoreboard.Gametime` (`self.Scoreboard`)) (`KismetTextLibrary.Conv_StringToText` (`KismetStringLibrary.Concat_StrStr` (`KismetStringLibrary.Conv_IntToString` _returnvalue) ":" (`KismetStringLibrary.Conv_IntToString` (`KismetMathLibrary.Round` _remainder))))))

(event `UpdateShotClock`
  (bind _mymessagepopup (`/Game/Blueprints/Player/BaseCharacterController.MyMessagePopup` (`self.Player`)))
  (bind _returnvalue (`KismetMathLibrary.Round` (`KismetMathLibrary.FMod` (`KismetMathLibrary.Conv_IntToDouble` (- (`self.ShotClockLimit`) (`self.ShotClockTime`))) 60.0)))
  ;[1 1 1 1 24] Score
  (bind _output_get (set `self.ShotClockTime` (+ (`self.ShotClockTime`) 1)))
  (if (== _output_get (`self.ShotClockLimit`))
    (`self.ResetPlayGamemode` 0) ; ResetType: 0 = Shotclock, 1 = Score
    (`TextBlock.SetText` (`/Game/UI/UMG_MessagePopup.Line1` _mymessagepopup) "Shot Clock Violation!")
    (`Widget.SetVisibility` _mymessagepopup "Visible")
    (`KismetSystemLibrary.Delay` 0.5)
    (`Widget.SetVisibility` _mymessagepopup "Hidden")
    (elif (< _returnvalue 10)
      (`TextBlock.SetText` (`/Game/UI/UMG_Scoreboard.ShotClockTime` (`self.Scoreboard`)) (`KismetTextLibrary.Conv_StringToText` (`KismetStringLibrary.Concat_StrStr` "" ":0" (`KismetStringLibrary.Conv_IntToString` (`KismetMathLibrary.Round` (`KismetMathLibrary.FMod` (`KismetMathLibrary.Conv_IntToDouble` (- (`self.ShotClockLimit`) (`self.ShotClockTime`))) 60.0))))))
      (else
        (`TextBlock.SetText` (`/Game/UI/UMG_Scoreboard.ShotClockTime` (`self.Scoreboard`)) (`KismetTextLibrary.Conv_StringToText` (`KismetStringLibrary.Concat_StrStr` "" ":" (`KismetStringLibrary.Conv_IntToString` _returnvalue))))))))

(event `ResetPlayGamemode`
  (params (ResetType :type Integer))
  ;[1 1 1 1 24] Reset Play
  (`self.DetermineSides` ResetType))

(event `DetermineSides`
  (params (ResetType :type Integer))
  ;[1 1 1 1 24] Reset Play
  (switch `int` ResetType ; ResetType: 0 = Shotclock, 1 = Score, 2 = Out of Bounds
    (:`0`
      (`KismetSystemLibrary.PrintString` "PLAY RESET: Shot Clock")
      (set `self.bResetShotClock` true :!label _label)
      (`self.ResetPlayers` true))
    (:`1`
      (`KismetSystemLibrary.PrintString` "PLAY RESET: Score")
      (set `self.bResetShotClock` true)
      (`self.ResetPlayers` false :!label _label_2))
    (:`2`
      (`KismetSystemLibrary.PrintString` "PLAY RESET: Out of Bounds")
      (set `self.bResetShotClock` false)
      (goto _label_2))
    (:`3`
      (`KismetSystemLibrary.PrintString` "PLAY RESET: Steal Recovery")
      (goto _label))))

(event `ResetPlayers`
  (params (SwitchSides :type Boolean))
  ;[1 1 1 1 24] Reset Play
  (`/Game/Blueprints/Player/BaseCharacterController.ResetPlayPlayer` (`self.Player`) (`self.OffenseStartingPosition`) (`self.DefenseStartingPosition`) SwitchSides)
  (`/Game/Blueprints/AI/BaseAIController.ResetPlayAIPlayer` (`self.AI`) (`self.OffenseStartingPosition`) (`self.DefenseStartingPosition`) SwitchSides)
  (`/Game/Blueprints/Ball/BaseBall.ResetPlayBall` (`self.Ball`))
  (if (`self.bResetShotClock`)
    (`self.ResetShotclock`)))

(event `ResetShotclock`
  ;[1 1 1 1 24] Reset Play
  (set `self.ShotClockTime` 0))

(fn `UserConstructionScript`)