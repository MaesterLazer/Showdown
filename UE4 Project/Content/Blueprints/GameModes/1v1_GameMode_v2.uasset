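; Game mode for a 1v1 ball game that handles scoring and play resets between a player and an AI opponent.
; A score refreshes the scoreboard, currently with hardcoded zeros, then triggers a reset after a short delay.
; DetermineSides maps the reset reason to a side switch: shot clock timeout and steal recovery swap sides.
; ResetPlayers repositions both players and the ball via ShowdownGameState references, then restarts the shot clock.
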(event `self.ReceiveBeginPlay`
  ;[1 1 1 1 24] Begin Play
  (bind _asshowdown_game_state (cast `ShowdownGameState` (`GameplayStatics.GetGameState`)))
  (set `self.GameStateRef` _asshowdown_game_state))

(event `ShowdownInterface.EventScore`
  ;[1 1 1 1 24] Score
  (`self.Update Scoreboard`)
  (`KismetSystemLibrary.Delay` 0.2)
  (`self.DetermineSides` "Score"))

(event `Update Scoreboard`
  ;[1 1 1 1 24] Score
  (`TextBlock.SetText` (`/Game/UI/UMG_Scoreboard.Score` (`self.Scoreboard`)) (`KismetTextLibrary.Conv_StringToText` (`KismetStringLibrary.Concat_StrStr` (`KismetStringLibrary.Conv_IntToString` 0) " - " (`KismetStringLibrary.Conv_IntToString` 0))))
  (`KismetSystemLibrary.Delay` 1.0))

(event `DetermineSides`
  (params (ResetType :type "E_GameplayEvent Enum" :default "Score"))
  ;[1 1 1 1 24] Reset Play
  (switch `E_GameplayEvent` ResetType
    (:`Score`
      (`KismetSystemLibrary.PrintString` "PLAY RESET: Score")
      (`self.ResetPlayers` false true))
    (:`ShotClockTimeOut`
      (`KismetSystemLibrary.PrintString` "PLAY RESET: Shot Clock")
      (`self.ResetPlayers` true true :!label _label))
    (:`OutOfBounds`
      (`KismetSystemLibrary.PrintString` "PLAY RESET: Out of Bounds")
      (`self.ResetPlayers` false true))
    (:`StealRecovery`
      (`KismetSystemLibrary.PrintString` "PLAY RESET: Steal Recovery")
      (goto _label))))

(event `ResetPlayers`
  (params (SwitchSides :type Boolean) (ShotClockReset :type Boolean))
  (bind (_gameobjects_homestartpos _gameobjects_awaystartpos _gameobjects_ballstartpos _gameobjects_hoop _gameobjects_homeplayer _gameobjects_awayplayer _gameobjects_ball) (break `GameplayObjects` (`ShowdownGameState.gameObjects` (`self.GameStateRef`))))
  (bind (_gameobjects_homestartpos_2 _gameobjects_awaystartpos_2 _gameobjects_ballstartpos_2 _gameobjects_hoop_2 _gameobjects_homeplayer_2) (break `GameplayObjects` (`ShowdownGameState.gameObjects` (`self.GameStateRef`))))
  ;[1 1 1 1 24] Reset Play
  (`/Game/Blueprints/Player/BaseCharacterController_v2.ResetPlayPlayer` (cast `/Game/Blueprints/Player/BaseCharacterController_v2` _gameobjects_homeplayer_2 :!pure true) _gameobjects_homestartpos_2 _gameobjects_awaystartpos_2 SwitchSides)
  (`/Game/Blueprints/AI/BaseAIController_v2.ResetPlayAIPlayer` (cast `/Game/Blueprints/AI/BaseAIController_v2` (`AIBlueprintHelperLibrary.GetAIController` (cast `/Game/Blueprints/AI/BaseAI_v2` _gameobjects_awayplayer :!pure true)) :!pure true) _gameobjects_homestartpos _gameobjects_awaystartpos SwitchSides)
  (`/Game/Blueprints/Ball/BaseBall_v2.ResetPlayBall` (cast `/Game/Blueprints/Ball/BaseBall_v2` _gameobjects_ball :!pure true))
  (if ShotClockReset
    (message `ShowdownInterface.EventOnShotClockStart` (`GameplayStatics.GetGameState`))))

(fn `UserConstructionScript`)