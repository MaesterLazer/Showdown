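; Game state for a 1v1 mode with a hoop, ball, home player and AI-driven away player.
; When game objects are registered, it passes the GameObjects set to the hoop, home player and ball through a registration message.
; For the away player, it casts to BaseAI and sends the message to that pawn's AI controller instead of the pawn.
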(event `self.EventOnRegisterGameObjects`
  (params (newGameObjects :type "GameplayObjects Structure"))
  (bind ((`Hoop` _hoop) (`HomePlayer` _homeplayer) (`AwayPlayer` _awayplayer) (`Ball` _ball)) (break `GameplayObjects` newGameObjects))
  (message `ShowdownInterface.EventOnRegisterGameObjects` _hoop (`self.gameObjects`))
  (message `ShowdownInterface.EventOnRegisterGameObjects` _homeplayer (`self.gameObjects`))
  (message `ShowdownInterface.EventOnRegisterGameObjects` (`AIBlueprintHelperLibrary.GetAIController` (cast `/Game/Blueprints/AI/BaseAI` _awayplayer :!pure true)) (`self.gameObjects`))
  (message `ShowdownInterface.EventOnRegisterGameObjects` _ball (`self.gameObjects`)))

(fn `UserConstructionScript`)