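; BaseHoop is a basketball hoop actor that awards a score when a ball overlaps it.
; On BeginPlay it casts the game mode to 1v1 and caches it, printing a message if the cast fails.
; On overlap it accepts only actors whose class is exactly BaseBall, then passes the ball's ShootingTeam to the game mode's AddScore.
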(event `self.ReceiveBeginPlay`
  ;[1 1 1 1 24] Startup
  (`self.DefineGamemode`))

(event `DefineGamemode`
  ;[1 1 1 1 24] Startup
  (bind _as1v_1 (cast `/Game/Blueprints/GameModes/1v1` (`GameplayStatics.GetGameMode`))
    (:`then`
      (set `self.Gamemode` _as1v_1))
    (:`CastFailed`
      (`KismetSystemLibrary.PrintString` "Failed GM Cast"))))

(event `self.ReceiveActorBeginOverlap`
  (params (OtherActor :type "Actor Object Reference"))
  ;[1 1 1 1 24] Score Check
  (if (== (`GameplayStatics.GetObjectClass` OtherActor) "/Game/Blueprints/Ball/BaseBall.BaseBall_C")
    (bind _asbase_ball (cast `/Game/Blueprints/Ball/BaseBall` OtherActor))
    (`/Game/Blueprints/GameModes/1v1.AddScore` (`self.Gamemode`) (`/Game/Blueprints/Ball/BaseBall.ShootingTeam` _asbase_ball))))

(fn `UserConstructionScript`)