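; BaseCharacter is the player character Blueprint, with a follow camera and ball pickup on overlap.
; When it overlaps a BaseBall_v2, it passes the ball to player 0's BaseCharacterController through BallPickupPlayer, regardless of which controller possesses the character.
; The construction script disables the camera's aspect ratio constraint and stores the skeletal mesh for socket use.
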(event `self.ReceiveActorBeginOverlap`
  (params (OtherActor :type "Actor Object Reference"))
  ;[1 1 1 1 28] Ball Overlap
  (bind _asbase_ball_v_2 (cast `/Game/Blueprints/Ball/BaseBall_v2` OtherActor))
  (if true
    (bind _asbase_character_controller (cast `/Game/Blueprints/Player/BaseCharacterController` (`GameplayStatics.GetPlayerController` 0)))
    (`/Game/Blueprints/Player/BaseCharacterController.BallPickupPlayer` _asbase_character_controller _asbase_ball_v_2)))

(fn `UserConstructionScript`
  (bind _followcamera (`self.FollowCamera`))
  (`|ExecutionSequence`
    (:`then_0`
      ;[1 1 1 1 28] Camera Aspect Ratio
      (`CameraComponent.SetAspectRatio` _followcamera 0.0)
      (`CameraComponent.SetConstraintAspectRatio` _followcamera false))
    (:`then_1`
      ;[1 1 1 1 28] Skeletal Mesh Reference (for sockets)
      (set `self.PlayerSkeletalMesh` (`self.Mesh`)))
    (:`then_2`)))