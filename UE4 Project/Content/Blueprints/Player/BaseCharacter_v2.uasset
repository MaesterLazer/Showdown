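; Player character for a basketball game, with separate offense and defense cameras and ball pickup on overlap.
; A 120 Hz looping timer tilts the offense camera by squared horizontal distance to the hoop while its controller is on offense and not resetting.
; Overlapping a ball passes it to the first player controller's pickup function.
; Construction caches both camera transforms for the reset event; camera side-switching logic is defunct.
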(event `self.ReceiveBeginPlay`
  ;[1 1 1] Begin Play
  (`KismetSystemLibrary.K2_SetTimerDelegate` (delegate `UpdateTilt`) (/ 1.0 120.0) true))

(event `UpdateTilt`
  (bind _followcamera (`self.FollowCamera`))
  ;[1 1 1] Begin Play
  (bind _asbase_character_controller_v_2 (cast `/Game/Blueprints/Player/BaseCharacterController_v2` (`self.GetController`)))
  (if (`/Game/Blueprints/Player/BaseCharacterController_v2.bIsResetting` _asbase_character_controller_v_2)
    _
    (elif (`/Game/Blueprints/Player/BaseCharacterController_v2.bOffense` _asbase_character_controller_v_2)
      (`SceneComponent.K2_SetRelativeRotation` _followcamera (`KismetMathLibrary.MakeRotator` (.roll (`SceneComponent.K2_GetComponentRotation` _followcamera)) (* -1 (`KismetMathLibrary.Lerp` -13.0 2.0 (/ (+ (`KismetMathLibrary.Square` (- (.x (`self.K2_GetActorLocation` (`/Game/Blueprints/Player/BaseCharacterController_v2.TheHoop` _asbase_character_controller_v_2))) (.x (`self.K2_GetActorLocation`)))) (`KismetMathLibrary.Square` (- (.y (`self.K2_GetActorLocation` (`/Game/Blueprints/Player/BaseCharacterController_v2.TheHoop` _asbase_character_controller_v_2))) (.y (`self.K2_GetActorLocation`))))) 800000.0))) (.yaw (`SceneComponent.K2_GetComponentRotation` _followcamera))) false false))))

(event `self.ReceiveActorBeginOverlap`
  (params (OtherActor :type "Actor Object Reference"))
  (bind _overlappingactors (`self.GetOverlappingActors` "/Game/Blueprints/Ball/BaseBall_v2.BaseBall_v2_C"))
  ;[1 1 1 1 28] Ball Overlap
  (if (!= (`KismetArrayLibrary.Array_Length` _overlappingactors) 0)
    (bind _asbase_ball_v_2 (cast `/Game/Blueprints/Ball/BaseBall_v2` (`|GetArrayItem` _overlappingactors)))
    (bind _asbase_character_controller_v_2 (cast `/Game/Blueprints/Player/BaseCharacterController_v2` (`GameplayStatics.GetPlayerController` 0)))
    (`/Game/Blueprints/Player/BaseCharacterController_v2.BallPickupPlayer` _asbase_character_controller_v_2 _asbase_ball_v_2)))

(event `ResetCameraTransforms`
  ;[1 1 1 1 28] CameraReset
  (`SceneComponent.K2_SetRelativeTransform` (`self.FollowCamera`) (`self.CameraOffenseInitialTransform`) false true)
  (`SceneComponent.K2_SetRelativeTransform` (`self.FollowCameraDefense`) (`self.CameraDefenseInitialTransform`) false true))

(event `CameraSwitchSidesCharacter`
  ;[1 1 1 1 28] Camera Management (INACTIVE)
)

(fn `UserConstructionScript`
  (bind _followcamera (`self.FollowCamera`))
  (`|ExecutionSequence`
    (:`then_0`
      ;[1 1 1 1 28] Camera Aspect Ratio
      (`CameraComponent.SetAspectRatio` _followcamera (`self.AspectRatio`))
      (`CameraComponent.SetConstraintAspectRatio` _followcamera false))
    (:`then_1`
      ;[1 1 1 1 28] Skeletal Mesh Reference (for sockets)
      (set `self.PlayerSkeletalMesh` (`self.Mesh`)))
    (:`then_2`
      ;[1 1 1 1 28] Get Camera Origins
      (set `self.CameraOffenseInitialTransform` (`SceneComponent.GetRelativeTransform` (`self.FollowCamera`)))
      (set `self.CameraDefenseInitialTransform` (`SceneComponent.GetRelativeTransform` (`self.FollowCameraDefense`))))))