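; Player controller that moves the controlled pawn and forwards number-key presses to the character as target changes.
; An UpdateAxis event stores an eight-way-plus-center direction, which MovePawnOnAxis converts every tick into movement input along the pawn's forward and right vectors.
; Keys 1 to 3 cast the pawn to Character and call ChangeTarget with a key index, with animation disabled only for the third.
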(event `self.ReceiveTick`
  (params (DeltaSeconds :type "Float (single-precision)"))
  (`self.MovePawnOnAxis`))

(event `UpdateAxis`
  (params (Axis :type String))
  (set `self.MovementAxis` Axis))

(event `Key|One`
  (params (Key :type "Key Structure"))
  (:`Pressed`
    (bind _ascharacter (cast `/Game/Blueprints/Player/Character` (`self.K2_GetPawn`)))
    (`/Game/Blueprints/Player/Character.Change Target` _ascharacter true 0)))

(event `Key|Two`
  (params (Key :type "Key Structure"))
  (:`Pressed`
    (bind _ascharacter (cast `/Game/Blueprints/Player/Character` (`self.K2_GetPawn`)))
    (`/Game/Blueprints/Player/Character.Change Target` _ascharacter true 1)))

(event `Key|Three`
  (params (Key :type "Key Structure"))
  (:`Pressed`
    (bind _ascharacter (cast `/Game/Blueprints/Player/Character` (`self.K2_GetPawn`)))
    (`/Game/Blueprints/Player/Character.Change Target` _ascharacter false 2)))

(fn `MovePawnOnAxis`
  (locals (ScaleX :type "Float (double-precision)" :default 0.0) (ScaleY :type "Float (double-precision)" :default 0.0) (DirectionX :type "Vector Structure" :default (0.0 0.0 0.0)) (DirectionY :type "Vector Structure" :default (0.0 0.0 0.0)))
  (switch `string` (`self.MovementAxis`)
    (:`N`
      (set `local.ScaleX` 0.0)
      (set `local.DirectionX` (0.0 0.0 0.0))
      (set `local.ScaleY` 1.0)
      (set `local.DirectionY` (`self.GetActorForwardVector` (`self.K2_GetPawn`))))
    (:`NE`
      (set `local.ScaleX` 1.0)
      (set `local.DirectionX` (`self.GetActorRightVector` (`self.K2_GetPawn`)))
      (set `local.ScaleY` 1.0)
      (set `local.DirectionY` (`self.GetActorForwardVector` (`self.K2_GetPawn`))))
    (:`E`
      (set `local.ScaleX` 1.0)
      (set `local.DirectionX` (`self.GetActorRightVector` (`self.K2_GetPawn`)))
      (set `local.ScaleY` 0.0)
      (set `local.DirectionY` (`self.GetActorForwardVector` (`self.K2_GetPawn`))))
    (:`SE`
      (set `local.ScaleX` 1.0)
      (set `local.DirectionX` (`self.GetActorRightVector` (`self.K2_GetPawn`)))
      (set `local.ScaleY` -1.0)
      (set `local.DirectionY` (`self.GetActorForwardVector` (`self.K2_GetPawn`))))
    (:`S`
      (set `local.ScaleX` 0.0)
      (set `local.DirectionX` (`self.GetActorRightVector` (`self.K2_GetPawn`)))
      (set `local.ScaleY` -1.0)
      (set `local.DirectionY` (`self.GetActorForwardVector` (`self.K2_GetPawn`))))
    (:`SW`
      (set `local.ScaleX` -1.0)
      (set `local.DirectionX` (`self.GetActorRightVector` (`self.K2_GetPawn`)))
      (set `local.ScaleY` -1.0)
      (set `local.DirectionY` (`self.GetActorForwardVector` (`self.K2_GetPawn`))))
    (:`W`
      (set `local.ScaleX` -1.0)
      (set `local.DirectionX` (`self.GetActorRightVector` (`self.K2_GetPawn`)))
      (set `local.ScaleY` 0.0)
      (set `local.DirectionY` (`self.GetActorForwardVector` (`self.K2_GetPawn`))))
    (:`NW`
      (set `local.ScaleX` -1.0)
      (set `local.DirectionX` (`self.GetActorRightVector` (`self.K2_GetPawn`)))
      (set `local.ScaleY` 1.0)
      (set `local.DirectionY` (`self.GetActorForwardVector` (`self.K2_GetPawn`))))
    (:`C`
      (set `local.ScaleX` 0.0)
      (set `local.DirectionX` (`self.GetActorRightVector` (`self.K2_GetPawn`)))
      (set `local.ScaleY` 0.0)
      (set `local.DirectionY` (`self.GetActorForwardVector` (`self.K2_GetPawn`)))))
  (`Pawn.AddMovementInput` (`self.K2_GetPawn`) (`local.DirectionX`) (`local.ScaleX`) false)
  (`Pawn.AddMovementInput` (`self.K2_GetPawn`) (`local.DirectionY`) (`local.ScaleY`) false))

(fn `UserConstructionScript`)