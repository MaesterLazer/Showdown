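; ShowdownBall is a physics ball actor that can be held on a socket and then launched.
; AttachTo snaps it to a named socket on a given parent component.
; LaunchAtTarget detaches it, enables physics simulation on its static mesh, and sets the linear velocity directly from the supplied vector.
; OnGameplayEvent only prints the received event name for debugging.
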(event `self.OnGameplayEvent`
  (params (Event :type "E_GameEvent Enum" :default "BasketMade"))
  (`KismetSystemLibrary.PrintString` (`KismetStringLibrary.Concat_StrStr` "BALL :: " (`|GetEnumeratorNameAsString` Event)) true true (struct :`R` 0.666667 :`G` 0.342282 :`B` 0.095193 :`A` 1.0)))

(event `LaunchAtTarget`
  (params (Result :type Integer) (InputPin :type "Vector Structure"))
  (set `self.Result` Result)
  (`self.K2_DetachFromActor` "KeepRelative")
  (`PrimitiveComponent.SetSimulatePhysics` (`self.StaticMesh`) true)
  (`PrimitiveComponent.SetPhysicsLinearVelocity` (`self.StaticMesh`) InputPin false "None"))

(fn `AttachTo`
  (params (Parent :type "SceneComponent Object Reference") (SocketName :type Name))
  (`self.K2_AttachToComponent` Parent SocketName "SnapToTarget" "KeepRelative" "KeepWorld"))

(fn `UserConstructionScript`)