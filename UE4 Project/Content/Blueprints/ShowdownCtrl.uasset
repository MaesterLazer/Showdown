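; ShowdownCtrl is the player's controller in a basketball showdown, randomizing base stats at BeginPlay and driving the player's ShowdownPawn.
; Gameplay events cache hoop, ball and start positions on Init, move the pawn by possession on drive start, and hide the action timer on timeouts or failures.
; Shots become miss, rim or swish and launch the ball along a suggested projectile arc, though miss and rim offsets are currently multiplied by zero.
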(event `self.ReceiveBeginPlay`
  (`KismetSystemLibrary.Delay` 0.2)
  (`self.SetGameStateRef`)
  (set `self.baseStats` (make `ShowdownPlayerStats` (`KismetMathLibrary.RandomFloatInRange` 0.0 0.75) (`KismetMathLibrary.RandomFloatInRange` 0.0 0.75) (`KismetMathLibrary.RandomFloatInRange` 0.0 0.75) (`KismetMathLibrary.RandomFloatInRange` 0.0 0.75) (`KismetMathLibrary.RandomFloatInRange` 0.0 0.75) (`KismetMathLibrary.RandomFloatInRange` 0.0 0.75)))
  (set `self.PlayerPawn` (cast `/Game/Blueprints/ShowdownPawn` (`GameplayStatics.GetPlayerPawn` 0) :!pure true)))

(event `self.OnGameplayEvent`
  (params (Event :type "E_GameEvent Enum" :default "BasketMade"))
  (`parent.OnGameplayEvent` Event)
  (`self.OnGameEvent` Event)
  (`KismetSystemLibrary.PrintString` (`KismetStringLibrary.Concat_StrStr` "PLYR CTRL :: " (`|GetEnumeratorNameAsString` Event)) true true (struct :`R` 0.34598 :`G` 0.666667 :`A` 1.0)))

(event `OnShoot`
  (params (bSuccess :type Boolean))
  (if bSuccess
    (set `self.ShotResult` (`KismetMathLibrary.RandomIntegerInRange` 1 2))
    (else
      (set `self.ShotResult` 0)))
  (switch `int` (`self.ShotResult`) ; 0 = Fail, 1 = Bounce, 2 = Swish
    (:`0`
      (`KismetSystemLibrary.PrintString` "Miss") ; Randomly deviate shot target to miss
      (bind _outlaunchvelocity (`GameplayStatics.SuggestProjectileVelocity_CustomArc` (`self.K2_GetActorLocation` (`self.BasketBall`)) (`KismetMathLibrary.MakeVector` (+ (.x (`self.HoopTarget`)) (* 0 (`KismetMathLibrary.RandomFloatInRange` 30.0 50.0))) (+ (.y (`self.HoopTarget`)) (* 0 (`KismetMathLibrary.RandomFloatInRange` 10.0 20.0))) (.z (`self.HoopTarget`))) 0.0 (`self.ShotArc`)))
      (set `self.ShotVelocity` _outlaunchvelocity))
    (:`1`
      (`KismetSystemLibrary.PrintString` "Tip") ; Randomly deviate shot target to hit rim
      (bind _outlaunchvelocity_2 (`GameplayStatics.SuggestProjectileVelocity_CustomArc` (`self.K2_GetActorLocation` (`self.BasketBall`)) (`KismetMathLibrary.MakeVector` (+ (.x (`self.HoopTarget`)) (* 0 (`KismetMathLibrary.RandomFloatInRange` 2.0 4.0))) (+ (.y (`self.HoopTarget`)) (* 0 (`KismetMathLibrary.RandomFloatInRange` 2.0 4.0))) (.z (`self.HoopTarget`))) 0.0 (`self.ShotArc`)))
      (set `self.ShotVelocity` _outlaunchvelocity_2))
    (:`2`
      (`KismetSystemLibrary.PrintString` "Swish")
      (bind _outlaunchvelocity_3 (`GameplayStatics.SuggestProjectileVelocity_CustomArc` (`self.K2_GetActorLocation` (`self.BasketBall`)) (`self.HoopTarget`) 0.0 (`self.ShotArc`)))
      (set `self.ShotVelocity` _outlaunchvelocity_3)))
  (`/Game/Blueprints/ShowdownBall.LaunchAtTarget` (`self.BasketBall`) (`self.ShotResult`) (`self.ShotVelocity`)))

(event `MoveToStartPos`
  (bind _returnvalue (`self.GetPossession`))
  (if _returnvalue
    (set `self.Move Target Pos` (`self.Offense Start Pos`))
    (else
      (set `self.Move Target Pos` (`self.Defense Start Pos`))))
  (`/Game/Blueprints/ShowdownPawn.MoveToLocation` (`self.PlayerPawn`) (`self.Move Target Pos`)))

(event `self.OnStunEffect`
  (params (bDisableEffect :type Boolean))
  (`parent.OnStunEffect` bDisableEffect)
  (`KismetSystemLibrary.PrintString` (`KismetStringLibrary.Concat_StrStr` "disabled stun effect :" (`KismetStringLibrary.Conv_BoolToString` bDisableEffect)))
  (if bDisableEffect
    (`/Game/Blueprints/ShowdownPawn.TickActionTimer` (`self.PlayerPawn`))))

(fn `OnGameEvent`
  (params (Event :type "E_GameEvent Enum" :default "BasketMade"))
  (locals (Objs :type "GameplayObjects Structure"))
  (switch `E_GameEvent` Event
    (:`ShotClockTimeout`
      (`SceneComponent.SetHiddenInGame` (`/Game/Blueprints/ShowdownPawn.ActionTimer` (`self.PlayerPawn`)) true false :!label _label))
    (:`DriveStart`
      (`self.MoveToStartPos`))
    (:`ActionFailed`
      (goto _label))
    (:`ActionTimedOut`
      (goto _label))
    (:`Init`
      (bind _asshowdown_gs (cast `/Game/Blueprints/ShowdownGS` (`GameplayStatics.GetGameState`)))
      (bind _output_get (set `local.Objs` (`GameStateSDF.gameObjects` _asshowdown_gs)))
      (bind (_homestartpos _awaystartpos _ballstartpos _hoop _homeplayer _awayplayer _ball) (break `GameplayObjects` _output_get))
      (set `self.HoopTarget` (`self.K2_GetActorLocation` _hoop))
      (bind _asshowdown_ball (cast `/Game/Blueprints/ShowdownBall` _ball))
      (set `self.BasketBall` _asshowdown_ball)
      (set `self.Offense Start Pos` _homestartpos)
      (set `self.Defense Start Pos` _awaystartpos)))
  (return))

(fn `UserConstructionScript`)