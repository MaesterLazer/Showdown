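; Game state for a one-on-one basketball showdown between a home player and an away opponent, directing possessions, actions and shots.
; A gameplay event state machine relays events to the ball, player controller and opponent, chaining phases by re-firing events after delays.
; Drive start attaches the ball to the possessing side's hand socket.
; Home actions trigger a delayed opponent response, and action results reach the hoop and controllers, with missed shots changing possession.
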(event `self.OnGameplayEvent`
  (params (Event :type "E_GameEvent Enum" :default "BasketMade"))
  (bind (_homestartpos _awaystartpos _ballstartpos _hoop _homeplayer _awayplayer _ball) (break `GameplayObjects` (`self.gameObjects`)))
  (bind _output_get (set `self.LastEvent` Event))
  (`parent.OnGameplayEvent` _output_get)
  (`KismetSystemLibrary.PrintString` (`KismetStringLibrary.Concat_StrStr` "GameState :: " (`|GetEnumeratorNameAsString` (`self.LastEvent`))))
  (switch `E_GameEvent` (`self.LastEvent`)
    (:`BasketMade`
      (message `InterfaceSDF.OnGameplayEvent` (`self.BallRef`) "BasketMade")
      (`KismetSystemLibrary.Delay` 2.0)
      (`self.OnGameplayEvent` "DriveStart"))
    (:`ChangePossession`
      (`/Game/Blueprints/ShowdownBall.OnGameplayEvent` (`self.BallRef`) (`self.LastEvent`))
      (`KismetSystemLibrary.Delay` 0.2)
      (`self.OnGameplayEvent` "DriveStart"))
    (:`ShotClockTimeout`
      (`ControllerSDF.OnGameplayEvent` (`self.PlayerCtrl`) (`self.LastEvent`) :!label _label)
      (message `InterfaceSDF.OnGameplayEvent` (`self.AwayCtrl`) (`self.LastEvent`))
      (message `InterfaceSDF.OnGameplayEvent` (`self.BallRef`) (`self.LastEvent`))
      (if (`|EnumEquality` (`self.LastEvent`) "Init")
        (`KismetSystemLibrary.Delay` 1.0)
        (`self.OnGameplayEvent` "GameStart")
        (elif (`|EnumEquality` (`self.LastEvent`) "ShotClockTimeout")
          (`KismetSystemLibrary.Delay` 1.0)
          (`self.OnGameplayEvent` "ChangePossession"))))
    (:`DriveStart`
      (if (`|EnumEquality` (`self.LastEvent`) "DriveStart")
        (`self.AssignBallToPlayer`)
        (goto _label)
        (else
          (goto _label))))
    (:`AwaitingAction`
      (goto _label))
    (:`ActionFailed`
      (goto _label))
    (:`ActionTimedOut`
      (`KismetSystemLibrary.Delay` 0.2)
      (`self.OnStunPossessingPlayer` false)
      (`self.OnGameplayEvent` "ActionFailed"))
    (:`ActionSuccess`
      (goto _label))
    (:`GameStart`
      (`self.OnGameplayEvent` "ChangePossession"))
    (:`Init`
      (set `self.BallRef` (cast `/Game/Blueprints/ShowdownBall` _ball :!pure true))
      (set `self.PlayerCtrl` (cast `/Game/Blueprints/ShowdownCtrl` _homeplayer :!pure true))
      (set `self.AwayCtrl` (cast `/Game/Blueprints/ShowdownOpponent` (`.AwayPlayer` (break `GameplayObjects` (`self.gameObjects`))) :!pure true))
      (goto _label))))

(event `self.OnActionAttempt`
  (params (Action :type "ShowdownPlayerActionData Structure"))
  (bind (_actionstat _actiontimereamining _team _action) (break `ShowdownPlayerActionData` Action))
  (`parent.OnActionAttempt` Action)
  (`KismetSystemLibrary.PrintString` (`KismetStringLibrary.Concat_StrStr` (`KismetStringLibrary.Concat_StrStr` (`|GetEnumeratorNameAsString` _team) " Player Took Action  | ") (`|GetEnumeratorNameAsString` _action)))
  (if (`|EnumEquality` _team "Home")
    (`KismetSystemLibrary.Delay` 0.5)
    (`/Game/Blueprints/ShowdownOpponent.TakeAction` (`self.AwayCtrl`) (`|EnumEquality` (`self.possession`) "Away"))))

(event `self.OnActionSucess`
  (params (Action :type "E_PlayerActions Enum" :default "Fake"))
  (`parent.OnActionSucess` Action)
  (`KismetSystemLibrary.PrintString` (`KismetStringLibrary.Concat_StrStr` "Action Sucess :: " (`|GetEnumeratorNameAsString` Action)))
  (message `InterfaceSDF.OnActionSucess` (`.Hoop` (break `GameplayObjects` (`self.gameObjects`))) Action)
  (`ControllerSDF.OnActionSucess` (`self.PlayerCtrl`) Action)
  (if (and (`|EnumEquality` Action "Shoot") (`|EnumEquality` (`self.possession`) "Home"))
    (`/Game/Blueprints/ShowdownCtrl.OnShoot` (`self.PlayerCtrl`) true)
    (elif (and (`|EnumEquality` Action "Shoot") (`|EnumEquality` (`self.possession`) "Away"))
      (`/Game/Blueprints/ShowdownOpponent.OnShoot` (`self.AwayCtrl`) false))))

(event `self.OnActionFail`
  (params (bTimedOut :type Boolean) (Action :type "E_PlayerActions Enum" :default "Fake"))
  (`parent.OnActionFail` bTimedOut Action)
  (`KismetSystemLibrary.PrintString` (`KismetStringLibrary.Concat_StrStr` "Action Fail :: " (`|GetEnumeratorNameAsString` Action)))
  (message `InterfaceSDF.OnActionFail` (`.Hoop` (break `GameplayObjects` (`self.gameObjects`))) bTimedOut Action)
  (`ControllerSDF.OnActionFail` (`self.PlayerCtrl`) bTimedOut Action)
  (if (and (`|EnumEquality` Action "Shoot") (`|EnumEquality` (`self.possession`) "Home"))
    (`/Game/Blueprints/ShowdownCtrl.OnShoot` (`self.PlayerCtrl`) false)
    (`KismetSystemLibrary.Delay` 5.0 :!label _label_2)
    (`self.OnGameplayEvent` "ChangePossession")
    (elif (and (`|EnumEquality` Action "Shoot") (`|EnumEquality` (`self.possession`) "Away"))
      (`/Game/Blueprints/ShowdownOpponent.OnShoot` (`self.AwayCtrl`) false)
      (goto _label_2))))

(event `self.OnStunPossessingPlayer`
  (params (bDisableStun :type Boolean))
  (`self.StunPlayer` bDisableStun)
  (`parent.OnStunPossessingPlayer` bDisableStun))

(fn `AssignBallToPlayer`
  (bind _ballref (`self.BallRef`))
  (switch `E_Team` (`self.possession`)
    (:`Home`
      (`/Game/Blueprints/ShowdownBall.AttachTo` _ballref (`Character.Mesh` (`/Game/Blueprints/ShowdownCtrl.PlayerPawn` (`self.PlayerCtrl`))) "ballSocketR"))
    (:`Away`
      (`/Game/Blueprints/ShowdownBall.AttachTo` _ballref (`/Game/Blueprints/ShowdownOpponent.SkeletalMesh` (`self.AwayCtrl`)) "ballSocketR"))
    (:`Free`
      _))
  (return))

(fn `StunPlayer`
  (params (bStun :type Boolean))
  (locals (bDisableStun :type Boolean :default false))
  (bind _output_get (set `local.bDisableStun` bStun))
  (`ControllerSDF.OnStunEffect` (`self.PlayerCtrl`) _output_get)
  (return))

(fn `UserConstructionScript`)