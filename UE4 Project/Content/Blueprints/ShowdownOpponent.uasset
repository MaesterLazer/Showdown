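; AI opponent for a basketball showdown, with randomized stats and actions reported to GameStateSDF as the Away team.
; It shoots when in possession, otherwise randomly picks block, steal or psyche.
; Game events cache court objects on Init and lerp it to a start position on Drive Start.
; Shot results launch the ball on a suggested arc as miss, rim or swish, though miss and rim offsets are multiplied by zero.
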(event `self.ReceiveBeginPlay`
  (set `self.GameState` (cast `GameStateSDF` (`GameplayStatics.GetGameState`) :!pure true))
  (set `self.BaseStats` (make `ShowdownPlayerStats` (`KismetMathLibrary.RandomFloatInRange` 0.0 0.75) (`KismetMathLibrary.RandomFloatInRange` 0.0 0.75) (`KismetMathLibrary.RandomFloatInRange` 0.0 0.75) (`KismetMathLibrary.RandomFloatInRange` 0.0 0.75) (`KismetMathLibrary.RandomFloatInRange` 0.0 0.75) (`KismetMathLibrary.RandomFloatInRange` 0.0 0.75))))

(event `self.OnGameplayEvent`
  (params (Event :type "E_GameEvent Enum" :default "BasketMade"))
  (`self.OnGameEvent` Event)
  (`KismetSystemLibrary.PrintString` (`KismetStringLibrary.Concat_StrStr` "Opponent :: " (`|GetEnumeratorNameAsString` Event)) true true (struct :`R` 1.0 :`B` 0.004442 :`A` 1.0)))

(event `MoveToLocation`
  (if (`self.GetPoessession`)
    (set `self.NewPos` (`.HomeStartPos` (break `GameplayObjects` (`self.GameObjs`))))
    (bind (_direction _alpha) (`Timeline|TL_MoveToStart` :!via `PlayFromStart` :!label _label)
      (:`Update`
        (bind (_returnvalue_location _returnvalue_rotation) (`KismetMathLibrary.BreakTransform` (`KismetMathLibrary.TLerp` (`self.GetTransform`) (`self.NewPos`) _alpha)))
        (`self.K2_SetActorLocationAndRotation` _returnvalue_location _returnvalue_rotation)))
    (else
      (set `self.NewPos` (`.AwayStartPos` (break `GameplayObjects` (`self.GameObjs`))))
      (goto _label :!via `PlayFromStart`))))

(event `self.OnActionSucess`
  (params (Action :type "E_PlayerActions Enum" :default "Fake"))
  (if (`|EnumEquality` Action "Shoot")
    (`self.OnShoot` true)))

(event `self.OnActionFail`
  (params (bTimedOut :type Boolean) (Action :type "E_PlayerActions Enum" :default "Fake"))
  (if (`|EnumEquality` Action "Shoot")
    (`self.OnShoot` false)))

(event `OnShoot`
  (params (bSuccess :type Boolean))
  (if bSuccess
    (set `self.ShotResult` (`KismetMathLibrary.RandomIntegerInRange` 1 2))
    (else
      (set `self.ShotResult` 0)))
  (switch `int` (`self.ShotResult`) ; 0 = Fail, 1 = Bounce, 2 = Swish
    (:`0`
      (`KismetSystemLibrary.PrintString` "Miss") ; Randomly deviate shot target to miss
      (bind _outlaunchvelocity (`GameplayStatics.SuggestProjectileVelocity_CustomArc` (`self.K2_GetActorLocation` (`self.BasketBall`)) (`KismetMathLibrary.MakeVector` (+ (.x (`self.HoopTarget`)) (* 0 (`KismetMathLibrary.RandomFloatInRange` 30.0 50.0))) (+ (.y (`self.HoopTarget`)) (* 0 (`KismetMathLibrary.RandomFloatInRange` 10.0 20.0))) (.z (`self.HoopTarget`))) 0.0 (`self.ShotArc`)))
      (set `self.ShotVelocity` _outlaunchvelocity))
    (:`1`
      (`KismetSystemLibrary.PrintString` "Tip") ; Randomly deviate shot target to hit rim
      (bind _outlaunchvelocity_2 (`GameplayStatics.SuggestProjectileVelocity_CustomArc` (`self.K2_GetActorLocation` (`self.BasketBall`)) (`KismetMathLibrary.MakeVector` (+ (.x (`self.HoopTarget`)) (* 0 (`KismetMathLibrary.RandomFloatInRange` 2.0 4.0))) (+ (.y (`self.HoopTarget`)) (* 0 (`KismetMathLibrary.RandomFloatInRange` 2.0 4.0))) (.z (`self.HoopTarget`))) 0.0 (`self.ShotArc`)))
      (set `self.ShotVelocity` _outlaunchvelocity_2))
    (:`2`
      (`KismetSystemLibrary.PrintString` "Swish")
      (bind _outlaunchvelocity_3 (`GameplayStatics.SuggestProjectileVelocity_CustomArc` (`self.K2_GetActorLocation` (`self.BasketBall`)) (`self.HoopTarget`) 0.0 (`self.ShotArc`)))
      (set `self.ShotVelocity` _outlaunchvelocity_3)))
  (`/Game/Blueprints/ShowdownBall.LaunchAtTarget` (`self.BasketBall`) (`self.ShotResult`) (`self.ShotVelocity`)))

(fn `OnGameEvent`
  (params (Event :type "E_GameEvent Enum" :default "BasketMade"))
  (switch `E_GameEvent` Event
    (:`DriveStart`
      (`self.MoveToLocation`))
    (:`Init`
      (bind _asgame_state_sdf (cast `GameStateSDF` (`GameplayStatics.GetGameState`)))
      (bind _output_get (set `self.GameObjs` (`GameStateSDF.gameObjects` _asgame_state_sdf)))
      (bind (_homestartpos _awaystartpos _ballstartpos _hoop _homeplayer _awayplayer _ball) (break `GameplayObjects` _output_get))
      (set `self.HoopTarget` (`self.K2_GetActorLocation` _hoop))
      (set `self.BasketBall` (cast `/Game/Blueprints/ShowdownBall` _ball :!pure true))))
  (return))

(fn `TakeAction`
  (params (bHasPossession :type Boolean))
  (locals (ActionToTake :type "E_PlayerActions Enum"))
  (if bHasPossession
    (set `local.ActionToTake` "Shoot")
    (else
      (set `local.ActionToTake` (select `int` (`KismetMathLibrary.RandomIntegerInRange` 0 2) :`0` "Block" :`1` "Steal" :`2` "Pysche" :!type "E_PlayerActions Enum"))))
  (`GameStateSDF.OnActionAttempt` (`self.GameState`) (make `ShowdownPlayerActionData` (`self.GetStatForAction` (`local.ActionToTake`)) (`GameStateSDF.actionTimerCount` (`self.GameState`)) "Away" (`local.ActionToTake`)))
  (return))

(fn `UserConstructionScript`)