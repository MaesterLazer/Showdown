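; Showdown pawn that owns the player's portrait 9:16 camera view, moves between locations and shows an action countdown.
; MoveToLocation lerps from the current transform to the target on a timeline, then signals AwaitingAction to GameState.
; TickActionTimer drives a dynamic material's Percent over a timeline sized to the GameMode's time limit.
; Its update lerp has zero alpha, so Percent holds at full until dropping to zero on finish.
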(event `TickActionTimer`
  (`MaterialInstanceDynamic.SetScalarParameterValue` (`self.TimerMat`) "Percent" 1.0)
  (`SceneComponent.SetHiddenInGame` (`self.ActionTimer`) false false)
  (`Timeline|TL_TickTimer` :!via `PlayFromStart`
    (:`Update`
      (bind _returnvalue (`MaterialInstanceDynamic.K2_GetScalarParameterValue` (`self.TimerMat`) "Percent"))
      (`MaterialInstanceDynamic.SetScalarParameterValue` (`self.TimerMat`) "Percent" (`KismetMathLibrary.Lerp` _returnvalue (/ (`GameStateSDF.actionTimerCount` (`self.GameState`)) (`self.TimerLimit`)))))
    (:`Finished`
      (`MaterialInstanceDynamic.SetScalarParameterValue` (`self.TimerMat`) "Percent" 0.0))))

(event `MoveToLocation`
  (params (TargetPos :type "Transform Structure"))
  (set `self.NewPos` TargetPos)
  (bind (_direction _lerpalpha) (`Timeline|TL_MoveToLoc` :!via `PlayFromStart`)
    (:`Update`
      (bind (_returnvalue_location _returnvalue_rotation) (`KismetMathLibrary.BreakTransform` (`KismetMathLibrary.TLerp` (`self.GetTransform`) (`self.NewPos`) _lerpalpha)))
      (`SceneComponent.K2_SetWorldLocationAndRotation` (`self.DefaultSceneRoot`) _returnvalue_location _returnvalue_rotation false false))
    (:`Finished`
      (`GameStateSDF.OnGameplayEvent` (`self.GameState`) "AwaitingAction"))))

(event `self.ReceiveBeginPlay`
  (bind _camera (`self.Camera`))
  (bind _asgame_state_sdf (cast `GameStateSDF` (`GameplayStatics.GetGameState`)))
  (set `self.GameState` _asgame_state_sdf)
  (`PlayerController.SetViewTargetWithBlend` (`GameplayStatics.GetPlayerController` 0) (`ActorComponent.GetOwner` (`self.Camera`)) 0.0 "VTBlend_Linear" 0.0 false)
  (`CameraComponent.SetConstraintAspectRatio` _camera true)
  (`CameraComponent.SetAspectRatio` _camera 0.5625)
  (`CameraComponent.SetFieldOfView` _camera 70.0)
  (bind _output_get (set `self.TimerLimit` (`GameModeSDF.actionTimerLimit` (cast `GameModeSDF` (`GameplayStatics.GetGameMode`) :!pure true))))
  (`TimelineComponent.SetTimelineLength` (`self.TL_TickTimer`) _output_get)
  (bind _returnvalue (`KismetMaterialLibrary.CreateDynamicMaterialInstance` "/Game/Materials/MAT_ActionTimer.MAT_ActionTimer"))
  (bind _output_get_2 (set `self.TimerMat` _returnvalue))
  (`PrimitiveComponent.SetMaterial` (`self.ActionTimer`) 0 _output_get_2)
  (`MaterialInstanceDynamic.SetScalarParameterValue` (`self.TimerMat`) "Percent" 1.0))

(fn `UserConstructionScript`)