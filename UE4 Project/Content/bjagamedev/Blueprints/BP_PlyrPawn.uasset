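; Player pawn for a touch-controlled basketball game, using UTC components for a movement joystick and a shoot tap area.
; Overlapping a BP_Ball attaches it to a hand socket and sets Possession.
; Shooting (tap, release or S key) jumps and switches AnimState; with the ball, it detaches and tweens it to above HoopLocation via MoveComponentTo.
; Arc-velocity and impulse shot experiments remain unconnected.
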(event `self.ReceiveBeginPlay`
  (bind _shootblock (`self.ShootBlock`))
  (`|ExecutionSequence`
    (:`then_0`
      (`/Game/UltimateTouchComponents/Core/UTCJoystickComponent.Setup Widget` (`self.MoveJoy`) (`self.JoyWidget`) true true))
    (:`then_1`
      (`/Game/UltimateTouchComponents/Core/UTCComponent.Setup Bounds` _shootblock true (0.8 0.7) (0.0 0.2) true true)
      (`/Game/UltimateTouchComponents/Core/UTCComponent.Setup Background by Bounds` _shootblock (`self.ShootBlockWidget`) true)
      (`UserWidget.SetColorAndOpacity` (`/Game/UltimateTouchComponents/Core/UTCComponent.Background Widget` (`self.ShootBlock`)) (struct :`R` 1.0 :`G` 1.0 :`B` 1.0 :`A` 0.45)))))

(event `InputTouch`
  (params (Location :type "Vector Structure") (FingerIndex :type "ETouchIndex Enum"))
  ;[1 0 0] Pass required events to all UTC components
  (:`Pressed`
    (`/Game/UltimateTouchComponents/Core/UTCMacroLibrary.UTC Touch Input Manager` Location FingerIndex :!label _label))
  (:`Released`
    (goto _label :!via `Released`))
  (:`Moved`
    (goto _label :!via `Moved`)))

(event `self.ReceivePossessed`
  (params (NewController :type "Controller Object Reference"))
  ;[1 0 0] Pass required events to all UTC components
  (`/Game/UltimateTouchComponents/Core/UTCMacroLibrary.UTC Pawn Possesion Manager` NewController (stale `self.ReceiveUnpossessed` OldController) :!label _label_2))

(event `self.ReceiveUnpossessed`
  (params (OldController :type "Controller Object Reference"))
  ;[1 0 0] Pass required events to all UTC components
  (goto _label_2 :!via `Unpossesed`))

(event `self.MoveJoy.On X Axis Changed`
  (params (Value :type "Float (single-precision)"))
  ;[0 1 0] Movement
  (`self.AddMovementInput` (1.0 0.0 0.0) (* Value -1.0)))

(event `self.MoveJoy.On Y Axis Changed`
  (params (Value :type "Float (single-precision)"))
  ;[0 1 0] Movement
  (`self.AddMovementInput` (0.0 1.0 0.0) Value))

(event `self.CapsuleComponent.OnComponentBeginOverlap`
  (params (OverlappedComponent :type "PrimitiveComponent Object Reference") (OtherActor :type "Actor Object Reference") (OtherComp :type "PrimitiveComponent Object Reference") (OtherBodyIndex :type Integer) (bFromSweep :type Boolean) (SweepResult :type "HitResult Structure (by ref)"))
  (bind _asbp_ball (cast `/Game/bjagamedev/Blueprints/BP_Ball` OtherActor))
  (set `self.BP_Ball` _asbp_ball)
  (`PrimitiveComponent.SetSimulatePhysics` (`/Game/bjagamedev/Blueprints/BP_Ball.Main` (`self.BP_Ball`)) false)
  (`/Game/bjagamedev/Blueprints/BP_Ball.AttachTo` (`self.BP_Ball`) (`self.Mesh`) "ballSocketR")
  (set `self.bPossession` true))

(event `self.ShootBlock.On Tap`
  (params (Location :type "Vector Structure") (FingerIndex :type "ETouchIndex Enum" :default "Touch1"))
  (`UserWidget.SetColorAndOpacity` (`/Game/UltimateTouchComponents/Core/UTCComponent.Background Widget` (`self.ShootBlock`)) (struct :`R` 1.0 :`G` 1.0 :`B` 1.0 :`A` 1.0))
  (`self.OnShoot` :!label _label_3))

(event `self.ShootBlock.On Tap Release`
  (params (Location :type "Vector Structure") (FingerIndex :type "ETouchIndex Enum" :default "Touch1"))
  (`UserWidget.SetColorAndOpacity` (`/Game/UltimateTouchComponents/Core/UTCComponent.Background Widget` (`self.ShootBlock`)) (struct :`R` 1.0 :`G` 1.0 :`B` 1.0 :`A` 0.45))
  (goto _label_3))

(event `OnShoot`
  (bind _bp_ball (`self.BP_Ball`))
  (bind _bp_ball_2 (`self.BP_Ball`))
  (if (`self.bPossession`) :!label _label_4
    (set `self.AnimState` "NewEnumerator4")
    (`self.Jump`)
    (`/Game/bjagamedev/Blueprints/BP_Ball.AttachTo` (`self.BP_Ball`) (`self.Mesh`) "ballSocketShoot")
    (`KismetSystemLibrary.Delay` 0.2)
    (set `self.AnimState` "NewEnumerator0")
    (set `self.bPossession` false)
    (set `ProjectileMovementComponent.bSimulationEnabled` true (`/Game/bjagamedev/Blueprints/BP_Ball.ProjectileMovement` _bp_ball_2))
    (`PrimitiveComponent.SetSimulatePhysics` (`/Game/bjagamedev/Blueprints/BP_Ball.Main` _bp_ball_2) true)
    (`self.K2_DetachFromActor` (`self.BP_Ball`) "KeepRelative" "KeepRelative" "KeepRelative")
    (`KismetSystemLibrary.MoveComponentTo` (`/Game/bjagamedev/Blueprints/BP_Ball.Main` _bp_ball) (+ (`KismetMathLibrary.VLerp` (`self.HoopLocation`) (`self.K2_GetActorLocation` (`self.BP_Ball`))) (0.0 0.0 70.0)) (struct :`Pitch` 5.0 :`Yaw` 10.0 :`Roll` 5.0) false true 0.6 :!label _label_5)
    ;[1 1 1] feeds into the stop; slight difference on the fall of the ball
    (`PrimitiveComponent.SetCollisionEnabled` (`/Game/bjagamedev/Blueprints/BP_Ball.Main` _bp_ball) "QueryAndPhysics")
    (goto _label_5 :!via `Stop`)
    (else
      (set `self.AnimState` "NewEnumerator6")
      (`self.Jump`)
      (`KismetSystemLibrary.Delay` 0.5)
      (set `self.AnimState` "NewEnumerator1"))))

(event `Key|S`
  (params (Key :type "Key Structure"))
  (:`Pressed`
    (goto _label_4)))

(fn `GetIsIdle`
  (returns (Idle :type "/Game/bjagamedev/AI/NPC_State Enum"))
  (bind _animstate (`self.AnimState`))
  (if (`self.bPossession`)
    (if (`|EnumEquality` _animstate "NewEnumerator0")
      (return "NewEnumerator0")
      (else
        (if (`|EnumEquality` _animstate "NewEnumerator1") :!label _label
          (return "NewEnumerator0"))))
    (else
      (goto _label))))

(fn `GetTeamID`
  (returns (IsPlayer :type Boolean))
  (return true))

(fn `UserConstructionScript`)