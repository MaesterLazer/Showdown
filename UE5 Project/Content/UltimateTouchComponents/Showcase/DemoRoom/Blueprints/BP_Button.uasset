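; BP_Button is a demo-room pressure button that animates when overlapped and switches a target Blueprint on or off.
; Trigger overlap plays the Press timeline and end overlap reverses it, driving the button's Z position and emissive glow through a dynamic material created in the construction script.
; When the timeline finishes, its direction sets the boolean sent to the target's ToggleMessage interface and to CallToggleEvent.
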(event `self.Trigger.OnComponentBeginOverlap`
  (params (OverlappedComponent :type "PrimitiveComponent Object Reference") (OtherActor :type "Actor Object Reference") (OtherComp :type "PrimitiveComponent Object Reference") (OtherBodyIndex :type Integer) (bFromSweep :type Boolean) (SweepResult :type "HitResult Structure (by ref)"))
  (bind _target_blueprint (`self.Target Blueprint`))
  (bind (_direction _press _glow) (`Timeline|Press` :!label _label) ; Timeline for animating the button press
    (:`Update`
      (`SceneComponent.K2_SetRelativeLocation` (`self.Button`) (`KismetMathLibrary.MakeVector` 0.0 0.0 _press) false false) ; Move button up/down
      (`MaterialInstanceDynamic.SetVectorParameterValue` (`self.Button material`) "Emissive" (`KismetMathLibrary.LinearColorLerp` (struct) (struct :`R` 0.6 :`G` 0.329323 :`A` 1.0) _glow)) ; Change emissive color of the button
    )
    (:`Finished`
      (if (`|EnumEquality` _direction "Forward")
        (message `/Game/UltimateTouchComponents/Showcase/DemoRoom/Blueprints/BPI_Interactions.Toggle` _target_blueprint true) ; Triggers a blueprint interface event in the target blueprint and sends it the "on/off" boolean
        (`self.ToggleEvent` true)
        (else
          (message `/Game/UltimateTouchComponents/Showcase/DemoRoom/Blueprints/BPI_Interactions.Toggle` _target_blueprint false) ; Triggers the same event, but this time the bool is false
          (`self.ToggleEvent` false))))))

(event `self.Trigger.OnComponentEndOverlap`
  (params (OverlappedComponent :type "PrimitiveComponent Object Reference") (OtherActor :type "Actor Object Reference") (OtherComp :type "PrimitiveComponent Object Reference") (OtherBodyIndex :type Integer))
  (goto _label :!via `Reverse`))

(fn `UserConstructionScript`
  (bind _returnvalue (`PrimitiveComponent.CreateDynamicMaterialInstance` (`self.Button`) 0 null)) ; Make and apply a dynamic material instance for the button
  (set `self.Button material` _returnvalue) ; Set the material as a variable for animating
)