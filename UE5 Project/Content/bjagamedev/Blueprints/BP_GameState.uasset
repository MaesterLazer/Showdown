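; BP_GameState tracks an AI wear-down bar that acts as a timed win condition for the AI.
; A looping one-second timer started on BeginPlay calls TickTimer, which raises the bar by a small fixed step.
; Tick polls the bar and, once it is full, uses a DoOnce to print an "AI WINS" debug message.
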(event `self.ReceiveBeginPlay`
  (`KismetSystemLibrary.K2_SetTimer` self "TickTimer" 1.0 true))

(event `self.ReceiveTick`
  (params (DeltaSeconds :type "Float (single-precision)"))
  (if (>= (`self.AIWeardownBar`) 1.0)
    (`/Engine/EditorBlueprintResources/StandardMacros.DoOnce` false
      (:`Completed`
        (`KismetSystemLibrary.PrintString` "AI WINS" true true (struct :`R` 0.604167 :`G` 0.090075 :`A` 1.0) 999.0)))))

(fn `TickTimer`
  (set `self.AIWeardownBar` (+ (`self.AIWeardownBar`) 0.01)))

(fn `UserConstructionScript`)