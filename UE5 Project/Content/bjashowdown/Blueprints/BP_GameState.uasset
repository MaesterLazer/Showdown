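; Game state for a one-on-one basketball match between the player (Home) and an AI opponent (Away), tracking score, possession and out-of-bounds.
; Delayed gameplay events drive the phases and broadcast to both players and UI.
; Shoot, block and steal attempts resolve by random roll, weighted by stat comparison and hoop distance; the Away branch reuses Home >= Away unmirrored.
; Scores shift the AI weardown bar, and emptying it declares a player win.
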(event `self.ReceiveTick`
  (params (DeltaSeconds :type "Float (single-precision)"))
  ;[1 1 1] Tick
  (if (<= (`self.AIWeardownBar`) 0.0)
    (`/Engine/EditorBlueprintResources/StandardMacros.DoOnce` false
      (:`Completed`
        (`KismetSystemLibrary.PrintString` "PLAYER WINS" true true (struct :`R` 0.604167 :`G` 0.090075 :`A` 1.0) 999.0)
        (`self.OnGameplayEvent` "NewEnumerator10")))))

(event `self.OnGameplayEvent`
  (params (Event :type "/Game/bjashowdown/Blueprints/GameEvent Enum" :default "NewEnumerator0"))
  (bind _output_get (set `self.CurrentGameState` Event))
  (`KismetSystemLibrary.Delay` (`self.TimeDelay`))
  (`self.GameplayEventResponse` _output_get))

(event `self.RegisterGameObjects`
  (params (Objects :type "/Game/bjashowdown/Blueprints/S_GameObjs Structure"))
  (bind _output_get (set `self.GameObjs` Objects))
  (bind ((`HomePlayer_6_A24972B1453130552AFA6C8A20BD0B30` _homeplayer) (`AIC_14_102040F54DEB752912FDED891A420296` _aic)) (break `/Game/bjashowdown/Blueprints/S_GameObjs` _output_get))
  (bind _asopponent_aic (cast `/Game/bjashowdown/AI/Opponent_AIC` _aic))
  (set `self.AiControl` _asopponent_aic)
  (bind _asbp_plyr_pawn (cast `/Game/bjashowdown/Blueprints/BP_PlyrPawn` _homeplayer)
    (:`then`
      (set `self.HomeStats` (`/Game/bjashowdown/Blueprints/BP_PlyrPawn.Stats` _asbp_plyr_pawn))
      (set `self.HomePlyr` _asbp_plyr_pawn)
      (bind _asbp_opponent (cast `/Game/bjashowdown/Blueprints/BP_Opponent` (`.AwayPlayer_7_28B2971F43A174EACA3B6994D3DE134B` (break `/Game/bjashowdown/Blueprints/S_GameObjs` (`self.GameObjs`))))
        (:`then`
          (set `self.AwayStats` (`/Game/bjashowdown/Blueprints/BP_Opponent.Stats` _asbp_opponent))
          (set `self.AwayPlyr` _asbp_opponent))
        (:`CastFailed`
          _)))
    (:`CastFailed`
      _))
  (`self.OnGameplayEvent` "NewEnumerator0"))

(event `self.ReadyUp`
  (params (Team :type "/Game/bjashowdown/Blueprints/Possession Enum" :default "NewEnumerator0"))
  (switch `/Game/bjashowdown/Blueprints/Possession` Team
    (:`NewEnumerator0`
      (set `self.bHomeReady` true))
    (:`NewEnumerator1`
      (set `self.bAwayReady` true)))
  (if (and (`self.bAwayReady`) (`self.bHomeReady`))
    (`self.OnChangePossession` (`self.CurrentPossession`))))

(event `self.AttemptAction`
  (params (Team :type "/Game/bjashowdown/Blueprints/Possession Enum" :default "NewEnumerator0") (ActionTaken :type "/Game/bjashowdown/Blueprints/PlayerActions Enum" :default "NewEnumerator0"))
  (`self.HandleActionAttempt` Team ActionTaken))

(event `ResetActions`)

(event `self.OnScore`
  (params (Team :type "/Game/bjashowdown/Blueprints/Possession Enum" :default "NewEnumerator0"))
  (switch `/Game/bjashowdown/Blueprints/Possession` Team
    (:`NewEnumerator0`
      (set `self.AIWeardownBar` (- (`self.AIWeardownBar`) (`self.BarChunkLength`)))
      (`/Engine/EditorBlueprintResources/StandardMacros.IncrementInt` (`self.HomeScore`)
        (:`  `
          _)))
    (:`NewEnumerator1`
      (set `self.AIWeardownBar` (+ (`self.AIWeardownBar`) (`self.BarChunkLength`)))
      (`/Engine/EditorBlueprintResources/StandardMacros.IncrementInt` (`self.AwayScore`)
        (:`  `
          _))))
  (`self.OnScore` (`self.MainUI`) "NewEnumerator0")
  (set `self.bAwayReady` false)
  (set `self.bHomeReady` false)
  (`self.ResetActions`)
  (`KismetSystemLibrary.Delay` 1.5)
  (`self.OnGameplayEvent` "NewEnumerator1"))

(event `self.OnChangePossession`
  (params (Possession :type "/Game/bjashowdown/Blueprints/Possession Enum" :default "NewEnumerator0"))
  (bind _output_get (set `self.CurrentPossession` Possession))
  (`self.OnChangePossession` (`self.AwayPlyr`) _output_get)
  (`self.OnChangePossession` (`self.HomePlyr`) _output_get))

(event `self.OnOOB`
  (params (OutofBounds :type Boolean))
  (set `/Game/bjashowdown/Blueprints/BP_Opponent.Out` OutofBounds (`self.AwayPlyr`))
  (set `/Game/bjashowdown/AI/Opponent_AIC.Out` OutofBounds (`self.AiControl`))
  (if OutofBounds
    (`/Game/bjashowdown/AI/Opponent_AIC.FigureOutShotLocation` (`self.AiControl`) true)
    (else
      (`/Game/bjashowdown/AI/Opponent_AIC.FigureOutShotLocation` (`self.AiControl`) false))))

(fn `DetermineActionResult`
  (locals (HomeStat :type "Float (double-precision)") (AwayStat :type "Float (double-precision)") (ActionWinner :type "/Game/bjashowdown/Blueprints/Possession Enum") (ActionLoser :type "/Game/bjashowdown/Blueprints/Possession Enum") (HomeAction :type "/Game/bjashowdown/Blueprints/PlayerActions Enum") (AwayAction :type "/Game/bjashowdown/Blueprints/PlayerActions Enum") (HomePlayer :type "Actor Object Reference") (AwayPlayer :type "Actor Object Reference") (AIC :type "Actor Object Reference"))
  (bind (_awaystats_athleticism _awaystats_accuracy _awaystats_defense) (break `/Game/bjashowdown/Blueprints/S_Stats` (`self.AwayStats`)))
  (bind _homeplyr (`self.HomePlyr`))
  (bind _awayplyr (`self.AwayPlyr`))
  (bind _awayplyr_2 (`self.AwayPlyr`))
  (bind _homeplyr_2 (`self.HomePlyr`))
  (bind (_gameobjs_homeplayer _gameobjs_awayplayer _gameobjs_hoop) (break `/Game/bjashowdown/Blueprints/S_GameObjs` (`self.GameObjs`)))
  (bind (_gameobjs_homeplayer_2 _gameobjs_awayplayer_2 _gameobjs_hoop_2) (break `/Game/bjashowdown/Blueprints/S_GameObjs` (`self.GameObjs`)))
  (bind (_homestats_athleticism _homestats_accuracy _homestats_defense) (break `/Game/bjashowdown/Blueprints/S_Stats` (`self.HomeStats`)))
  (bind _homeplyr_3 (`self.HomePlyr`))
  (bind (_awaystats_athleticism_2 _awaystats_accuracy_2 _awaystats_defense_2) (break `/Game/bjashowdown/Blueprints/S_Stats` (`self.AwayStats`)))
  (bind _aic (`local.AIC`))
  (bind _aic_2 (`local.AIC`))
  (bind _homeplyr_4 (`self.HomePlyr`))
  (bind _awayplyr_3 (`self.AwayPlyr`))
  (bind (_homestats_athleticism_2 _homestats_accuracy_2 _homestats_defense_2) (break `/Game/bjashowdown/Blueprints/S_Stats` (`self.HomeStats`)))
  (bind _value (`BlueprintMapLibrary.Map_Find` (`self.CurrentActions`) "NewEnumerator0"))
  (bind _value_2 (`BlueprintMapLibrary.Map_Find` (`self.CurrentActions`) "NewEnumerator1"))
  (bind (_value_3 _returnvalue) (`BlueprintMapLibrary.Map_Find` (`self.CurrentActions`) "NewEnumerator0"))
  (bind (_value_4 _returnvalue_2) (`BlueprintMapLibrary.Map_Find` (`self.CurrentActions`) "NewEnumerator1"))
  (bind _returnvalue_3 (>= (`KismetMathLibrary.Vector_Distance2D` (`self.K2_GetActorLocation` _gameobjs_homeplayer) (`self.K2_GetActorLocation` _gameobjs_hoop)) 800.0))
  (bind _returnvalue_4 (>= (`KismetMathLibrary.Vector_Distance2D` (`self.K2_GetActorLocation` _gameobjs_awayplayer_2) (`self.K2_GetActorLocation` _gameobjs_hoop_2)) 800.0))
  (if _returnvalue
    (set `local.HomeAction` _value_3)
    ;[1 1 1] TODO: add mods like distance from goal, weardown etc
    (switch `/Game/bjashowdown/Blueprints/PlayerActions` (`local.HomeAction`)
      (:`NewEnumerator0`
        (set `local.HomeStat` _homestats_accuracy)
        (set `local.AwayStat` _awaystats_accuracy))
      (:`NewEnumerator1`
        (set `local.HomeStat` _homestats_defense :!label _label)
        (set `local.AwayStat` _awaystats_defense))
      (:`NewEnumerator2`
        (goto _label)))
    (if (>= (`local.HomeStat`) (`local.AwayStat`))
      (if _returnvalue_3
        (switch `int` (`KismetMathLibrary.RandomIntegerInRange` 0 4) :!label _label_2
          (:`0`
            (switch `/Game/bjashowdown/Blueprints/PlayerActions` _value :!label _label_3
              (:`NewEnumerator0`
                (if (`/Game/bjashowdown/Blueprints/BPFL_Showdown.GetPossession` "NewEnumerator0")
                  (message `/Game/bjashowdown/Blueprints/BPI_Showdown.OnShootBasket` _homeplyr_2 true)
                  (`BlueprintMapLibrary.Map_Clear` (`self.CurrentActions`) :!label _label_4)
                  (return)))
              (:`NewEnumerator1`
                (`/Game/bjashowdown/Blueprints/BP_Opponent.SetBlocked` _awayplyr_3)
                (`self.OnBlocked` _awayplyr_3)
                (message `/Game/bjashowdown/Blueprints/BPI_Showdown.OnBlock` _homeplyr_2 true)
                (goto _label_4))
              (:`NewEnumerator2`
                (`/Game/bjashowdown/Blueprints/BP_Opponent.SetStolen` _awayplyr_3)
                (`self.OnStolen` _awayplyr_3)
                (`self.OnChangePossession` "NewEnumerator0")
                (message `/Game/bjashowdown/Blueprints/BPI_Showdown.OnSteal` _homeplyr_2 true)
                (goto _label_4))))
          (:`1`
            (switch `/Game/bjashowdown/Blueprints/PlayerActions` _value :!label _label_5
              (:`NewEnumerator0`
                (message `/Game/bjashowdown/Blueprints/BPI_Showdown.OnShootBasket` _homeplyr_3 false)
                (goto _label_4))
              (:`NewEnumerator1`
                (message `/Game/bjashowdown/Blueprints/BPI_Showdown.OnBlock` _homeplyr_3 false)
                (goto _label_4))
              (:`NewEnumerator2`
                (message `/Game/bjashowdown/Blueprints/BPI_Showdown.OnSteal` _homeplyr_3 false)
                (goto _label_4))))
          (:`2`
            (goto _label_5))
          (:`3`
            (goto _label_5))
          (:`4`
            (goto _label_3)))
        (else
          (switch `int` (`KismetMathLibrary.RandomIntegerInRange` 0 3)
            (:`0`
              (goto _label_3))
            (:`1`
              (goto _label_5))
            (:`2`
              (goto _label_5))
            (:`3`
              (goto _label_3)))))
      (elif _returnvalue_3
        (switch `int` (`KismetMathLibrary.RandomIntegerInRange` 0 6)
          (:`0`
            (goto _label_3))
          (:`1`
            (goto _label_5))
          (:`2`
            (goto _label_5))
          (:`3`
            (goto _label_5))
          (:`4`
            (goto _label_5))
          (:`5`
            (goto _label_5))
          (:`6`
            (goto _label_3)))
        (else
          (goto _label_2))))
    (elif _returnvalue_2
      (set `local.AwayAction` _value_4)
      (switch `/Game/bjashowdown/Blueprints/PlayerActions` (`local.AwayAction`)
        (:`NewEnumerator0`
          (set `local.AwayStat` _awaystats_accuracy_2)
          (set `local.HomeStat` _homestats_accuracy_2))
        (:`NewEnumerator1`
          (set `local.AwayStat` _awaystats_defense_2 :!label _label_6)
          (set `local.HomeStat` _homestats_defense_2))
        (:`NewEnumerator2`
          (goto _label_6)))
      (if (>= (`local.HomeStat`) (`local.AwayStat`))
        (if _returnvalue_4
          (switch `int` (`KismetMathLibrary.RandomIntegerInRange` 0 4) :!label _label_7
            (:`0`
              _)
            (:`1`
              (switch `/Game/bjashowdown/Blueprints/PlayerActions` _value_2 :!label _label_8
                (:`NewEnumerator0`
                  (message `/Game/bjashowdown/Blueprints/BPI_Showdown.OnShootBasket` _aic_2 false)
                  (message `/Game/bjashowdown/Blueprints/BPI_Showdown.OnShootBasket` _awayplyr_2 false)
                  (goto _label_4))
                (:`NewEnumerator1`
                  (message `/Game/bjashowdown/Blueprints/BPI_Showdown.OnBlock` _aic_2 false)
                  (message `/Game/bjashowdown/Blueprints/BPI_Showdown.OnBlock` _awayplyr_2 false)
                  (goto _label_4))
                (:`NewEnumerator2`
                  (message `/Game/bjashowdown/Blueprints/BPI_Showdown.OnSteal` _aic_2 false)
                  (message `/Game/bjashowdown/Blueprints/BPI_Showdown.OnSteal` _awayplyr_2 false)
                  (goto _label_4))))
            (:`2`
              (goto _label_8))
            (:`3`
              (goto _label_8))
            (:`4`
              _))
          (else
            (switch `int` (`KismetMathLibrary.RandomIntegerInRange` 0 3)
              (:`0`
                _)
              (:`1`
                (goto _label_8))
              (:`2`
                (goto _label_8))
              (:`3`
                _))))
        (elif _returnvalue_4
          (switch `int` (`KismetMathLibrary.RandomIntegerInRange` 0 6)
            (:`0`
              _)
            (:`1`
              (goto _label_8))
            (:`2`
              (goto _label_8))
            (:`3`
              (goto _label_8))
            (:`4`
              (goto _label_8))
            (:`5`
              (goto _label_8))
            (:`6`
              _))
          (else
            (goto _label_7))))
      (switch `/Game/bjashowdown/Blueprints/PlayerActions` _value_2
        (:`NewEnumerator0`
          (if (`/Game/bjashowdown/Blueprints/BPFL_Showdown.GetPossession` "NewEnumerator1")
            (message `/Game/bjashowdown/Blueprints/BPI_Showdown.OnShootBasket` _aic true)
            (message `/Game/bjashowdown/Blueprints/BPI_Showdown.OnShootBasket` _awayplyr true)
            (goto _label_4)))
        (:`NewEnumerator1`
          (`/Game/bjashowdown/Blueprints/BP_PlyrPawn.SetBlocked` _homeplyr_4)
          (`self.OnBlocked` _homeplyr)
          (message `/Game/bjashowdown/Blueprints/BPI_Showdown.OnBlock` _aic true)
          (message `/Game/bjashowdown/Blueprints/BPI_Showdown.OnBlock` _awayplyr true)
          (goto _label_4))
        (:`NewEnumerator2`
          (`/Game/bjashowdown/Blueprints/BP_PlyrPawn.SetStolen` _homeplyr_4)
          (`self.OnStolen` _homeplyr)
          (`self.OnChangePossession` "NewEnumerator1")
          (message `/Game/bjashowdown/Blueprints/BPI_Showdown.OnSteal` _aic true)
          (message `/Game/bjashowdown/Blueprints/BPI_Showdown.OnSteal` _awayplyr true)
          (goto _label_4)))
      (else
        (return)))))

(fn `GameplayEventResponse`
  (params (GameEvent :type "/Game/bjashowdown/Blueprints/GameEvent Enum" :default "NewEnumerator0"))
  (`/Game/bjashowdown/Blueprints/BPFL_Showdown.LogString` (`KismetStringLibrary.Concat_StrStr` "GameState Event ||" (`|GetEnumeratorNameAsString` (`local.GameEvent`))))
  (switch `/Game/bjashowdown/Blueprints/GameEvent` (`local.GameEvent`)
    (:`NewEnumerator0`
      (bind _output_get (set `self.CurrentGameState` "NewEnumerator1"))
      (`/Game/bjashowdown/Blueprints/BPFL_Showdown.LogString` (`KismetStringLibrary.Concat_StrStr` "GameState Event ||" (`|GetEnumeratorNameAsString` _output_get)))
      (`self.BroadcastGameEvent` _output_get)
      (set `self.CurrentPossession` "NewEnumerator0")
      (return))
    (:`NewEnumerator1`
      (bind _output_get_2 (set `self.CurrentGameState` "NewEnumerator1"))
      (`/Game/bjashowdown/Blueprints/BPFL_Showdown.LogString` (`KismetStringLibrary.Concat_StrStr` "GameState Event ||" (`|GetEnumeratorNameAsString` _output_get_2)))
      (`self.BroadcastGameEvent` _output_get_2))
    (:`NewEnumerator2`
      (bind _output_get_3 (set `self.CurrentGameState` "NewEnumerator2"))
      (`/Game/bjashowdown/Blueprints/BPFL_Showdown.LogString` (`KismetStringLibrary.Concat_StrStr` "GameState Event ||" (`|GetEnumeratorNameAsString` _output_get_3)))
      (`self.BroadcastGameEvent` _output_get_3)
      (return))
    (:`NewEnumerator3`
      (`/Game/bjashowdown/Blueprints/BPFL_Showdown.LogString` (`KismetStringLibrary.Concat_StrStr` "GameState Event ||" (`|GetEnumeratorNameAsString` (`local.GameEvent`))) :!label _label)
      (`self.BroadcastGameEvent` (`local.GameEvent`))
      (return))
    (:`NewEnumerator4`
      (goto _label))
    (:`NewEnumerator7`
      (`self.DetermineActionResult`)
      (return))
    (:`NewEnumerator9`
      (`self.BroadcastGameEvent` (`self.CurrentGameState`))
      (return))))

(fn `HandleActionAttempt`
  (params (Team :type "/Game/bjashowdown/Blueprints/Possession Enum (by ref)") (Action :type "/Game/bjashowdown/Blueprints/PlayerActions Enum (by ref)"))
  (`BlueprintMapLibrary.Map_Add` (`self.CurrentActions`) Team Action)
  (`self.OnGameplayEvent` "NewEnumerator7")
  (return))

(fn `TickTimer`
  (set `self.AIWeardownBar` (+ (`self.AIWeardownBar`) 0.01)))

(fn `UserConstructionScript`)