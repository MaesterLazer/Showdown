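; AI opponent character for a basketball game that picks up loose balls, shoots, steals and responds to blocks.
; Gameplay events and action results update its state for the anim instance, possession, blackboard and Opponent_AIC lock.
; An attached fake ball swaps for a projectile on shots or a physics pickup when blocked.
; Shots arc to a success point or random miss point, sequenced by delays and DoOnce gates.
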(event `self.ReceiveBeginPlay`
  (set `self.Stats` (make `/Game/bjashowdown/Blueprints/S_Stats` (`KismetMathLibrary.RandomFloatInRange` 0.0 1.0) (`KismetMathLibrary.RandomFloatInRange` 0.0 1.0) (`KismetMathLibrary.RandomFloatInRange` 0.0 1.0) (`KismetMathLibrary.RandomFloatInRange` 0.0 1.0))))

(event `self.NotifyStateChanged`
  (params (NewState :type "/Game/bjashowdown/Blueprints/NPC_State Enum" :default "NewEnumerator0"))
  ;[1 1 1] State Updates
  (bind _output_get (set `self.CurrentState` NewState))
  (message `/Game/bjashowdown/Shared/BPI_AI_Helper.NotifyStateChanged` (`SkeletalMeshComponent.GetAnimInstance` (`self.Mesh`)) _output_get))

(event `SetOffense`
  (`KismetSystemLibrary.Delay` 1.0)
  ;[1 1 1] Change this to IDLE if you don't want AI to go Offensive
  (bind _output_get (set `self.CurrentState` "NewEnumerator7"))
  (`self.NotifyStateChanged` _output_get))

(event `/Game/bjashowdown/Blueprints/BPI_Showdown.OnBlocked`
  (bind _ball (`self.Ball`))
  (bind _fakeball (`self.FakeBall`))
  (bind _returnvalue (`SceneComponent.K2_GetComponentToWorld` _fakeball))
  (if (`KismetSystemLibrary.IsValid` _ball)
    ;[1 1 1] Ball Blocked
    (`ProjectileMovementComponent.SetVelocityInLocalSpace` (`/Game/bjashowdown/Blueprints/BP_Ball.ProjectileMovement` _ball) (0.0 0.0 0.0))
    (`/Engine/EditorBlueprintResources/StandardMacros.DoOnce` false :!label _label
      (:`Completed`
        (bind _returnvalue_2 (`|SpawnActorFromClass` "/Game/bjashowdown/Blueprints/BP_FakeBall.BP_FakeBall_C" (`self.GetTransform` _ball) "Undefined" "OverrideRootScale" null null))
        (`PrimitiveComponent.SetSimulatePhysics` (`/Game/bjashowdown/Blueprints/BP_FakeBall.Main` _returnvalue_2) true)
        (set `/Game/bjashowdown/Blueprints/BP_PlyrPawn.BP_Faker` _returnvalue_2 (`self.Plyr`))
        (`self.K2_DestroyActor` (`self.Ball`))
        (bind _output_get (set `self.CurrentState` "NewEnumerator7"))
        (`self.NotifyStateChanged` _output_get)
        (`/Game/bjashowdown/AI/Opponent_AIC.EndLock` (`self.AIC`))
        (`KismetSystemLibrary.Delay` 0.5)
        (goto _label :!via `Reset`)))
    (else
      (`SceneComponent.SetVisibility` _fakeball false false)
      (`/Engine/EditorBlueprintResources/StandardMacros.DoOnce` false :!label _label_2
        (:`Completed`
          (bind _returnvalue_3 (`|SpawnActorFromClass` "/Game/bjashowdown/Blueprints/BP_FakeBall.BP_FakeBall_C" (`KismetMathLibrary.MakeTransform` (`KismetMathLibrary.MakeVector` (+ (.x (.location _returnvalue)) 50.0) (.y (.location _returnvalue)) (.z (.location _returnvalue))) (.rotation _returnvalue) (.scale _returnvalue)) "Undefined" "OverrideRootScale" null null))
          (`PrimitiveComponent.SetSimulatePhysics` (`/Game/bjashowdown/Blueprints/BP_FakeBall.Main` _returnvalue_3) true)
          (set `/Game/bjashowdown/Blueprints/BP_PlyrPawn.BP_Faker` _returnvalue_3 (`self.Plyr`))
          (bind _output_get_2 (set `self.CurrentState` "NewEnumerator7"))
          (`self.NotifyStateChanged` _output_get_2)
          (`/Game/bjashowdown/AI/Opponent_AIC.EndLock` (`self.AIC`))
          (`KismetSystemLibrary.Delay` 0.5)
          (goto _label_2 :!via `Reset`))))))

(event `self.CapsuleComponent.OnComponentBeginOverlap`
  (params (OverlappedComponent :type "PrimitiveComponent Object Reference") (OtherActor :type "Actor Object Reference") (OtherComp :type "PrimitiveComponent Object Reference") (OtherBodyIndex :type Integer) (bFromSweep :type Boolean) (SweepResult :type "HitResult Structure (by ref)"))
  (bind _aic (`self.AIC`))
  (if (not (`/Game/bjashowdown/Blueprints/BPFL_Showdown.GetPossession` (`self.Team`)))
    (bind _asbp_fake_ball (cast `/Game/bjashowdown/Blueprints/BP_FakeBall` OtherActor))
    (if (`KismetSystemLibrary.IsValid` _asbp_fake_ball)
      (message `/Game/bjashowdown/Blueprints/BPI_Showdown.OnChangePossession` (`GameplayStatics.GetGameState`) "NewEnumerator1")
      (`BlackboardComponent.SetValueAsBool` (`AIBlueprintHelperLibrary.GetBlackboard` null) (`self.BallStatus`) true)
      (`SceneComponent.K2_AttachToComponent` (`self.FakeBall`) (`self.Mesh`) "ballSocketR" "SnapToTarget" "KeepRelative" "KeepWorld" true)
      (`SceneComponent.SetVisibility` (`self.FakeBall`) true false)
      (`self.K2_DestroyActor` OtherActor)
      (`/Game/bjashowdown/AI/Opponent_AIC.SetReset` _aic false)
      (`/Game/bjashowdown/AI/Opponent_AIC.EndLock` _aic)
      (if (`self.Out`)
        (`/Game/bjashowdown/AI/Opponent_AIC.SetStateAsPossOOB` _aic)
        (else
          (`/Game/bjashowdown/AI/Opponent_AIC.SetStateAsShooting` _aic))))))

(event `/Game/bjashowdown/Blueprints/BPI_Showdown.OnStolen`
  ;[1 1 1] check for deprec
  (`SceneComponent.SetVisibility` (`self.FakeBall`) false false)
  ;;[1 1 1] For when the Player steals the ball from AI
  (`BlackboardComponent.SetValueAsBool` (`AIBlueprintHelperLibrary.GetBlackboard` null) (`self.BallStatus`) false)
  (bind _output_get (set `self.CurrentState` "NewEnumerator7"))
  (`self.NotifyStateChanged` _output_get)
  (`/Game/bjashowdown/AI/Opponent_AIC.EndLock` (`self.AIC`)))

(event `AtLocation`
  ;[1 1 1] check for deprec
  (`KismetSystemLibrary.Delay` 0.5)
  (bind _output_get (set `self.CurrentState` "NewEnumerator4"))
  (`self.NotifyStateChanged` _output_get))

(event `/Game/bjashowdown/Blueprints/BPI_Showdown.OnGameplayEvent`
  (params (Event :type "/Game/bjashowdown/Blueprints/GameEvent Enum" :default "NewEnumerator0"))
  (`self.OnGameEvent` Event))

(event `MoveToStartPos`
  (`KismetSystemLibrary.Delay` 0.2)
  (`/Game/bjashowdown/Blueprints/BPI_Showdown.ReadyUp` (`self.AIC`) "NewEnumerator1"))

(event `OnCheckBall`
  (bind _bhaspossession (`/Game/bjashowdown/Blueprints/BPFL_Showdown.GetPossession` (`self.Team`)))
  (`/Game/bjashowdown/Blueprints/BPFL_Showdown.LogString` (`KismetStringLibrary.Concat_StrStr` "AI CheckBall | HasPossession:  " (`KismetStringLibrary.Conv_BoolToString` _bhaspossession)))
  (if _bhaspossession
    _))

(event `ResetShooting`
  (bind _fakeball (`self.FakeBall`))
  (bind _fakeball_2 (`self.FakeBall`))
  (`|ExecutionSequence`
    (:`then_0`
      (`KismetSystemLibrary.Delay` 0.5)
      (goto _label_5 :!via `Reset`))
    (:`then_1`
      (`KismetSystemLibrary.Delay` 0.5)
      (goto _label_7 :!via `Reset`))
    (:`then_2`
      (`/Game/bjashowdown/AI/Opponent_AIC.ResetShoot` (`self.AIC`))
      (`KismetSystemLibrary.Delay` 0.5)
      (goto _label_3 :!via `Reset`))))

(event `/Game/bjashowdown/Blueprints/BPI_Showdown.OnShootBasket`
  (params (bSuccess :type Boolean))
  (bind _fakeball (`self.FakeBall`))
  (bind _fakeball_2 (`self.FakeBall`))
  (`/Game/bjashowdown/Blueprints/BPFL_Showdown.LogString` (`KismetStringLibrary.Concat_StrStr` "AI OnShoot | Sucess:  " (`KismetStringLibrary.Conv_BoolToString` bSuccess)))
  (`/Game/bjashowdown/Blueprints/BPFL_Showdown.LogString` (`KismetStringLibrary.Concat_StrStr` "AI OnShoot | HasPossession:  " (`KismetStringLibrary.Conv_BoolToString` (`/Game/bjashowdown/Blueprints/BPFL_Showdown.GetPossession` (`self.Team`)))))
  (`self.LookAtGoal`)
  (`/Game/bjashowdown/AI/Opponent_AIC.SetReset` (`self.AIC`) true)
  (`/Engine/EditorBlueprintResources/StandardMacros.DoOnce` false :!label _label_3
    (:`Completed`
      (if bSuccess
        (if (`/Game/bjashowdown/Blueprints/BPFL_Showdown.GetPossession` (`self.Team`))
          (if (or (`self.Stolen`) (`self.Blocked`))
            (`KismetSystemLibrary.Delay` 10.0 :!label _label_4)
            (set `self.Stolen` false)
            (set `self.Blocked` false)
            (`/Game/bjashowdown/AI/Opponent_AIC.EndLock` (`self.AIC`))
            (else
              ;[1 1 1] Shooting
              (if (`/Game/bjashowdown/Blueprints/BPFL_Showdown.GetPossession` (`self.Team`))
                (`/Engine/EditorBlueprintResources/StandardMacros.DoOnce` false :!label _label_5
                  (:`Completed`
                    (set `self.CurrentState` "NewEnumerator4")
                    ;[1 1 1] delay set for animation/behavior tree to fire
                    (`KismetSystemLibrary.Delay` 0.5)
                    (if (or (`self.Stolen`) (`self.Blocked`))
                      (goto _label_4)
                      (elif (`KismetSystemLibrary.IsValid` _fakeball)
                        (`SceneComponent.K2_AttachToComponent` _fakeball null "ballSocketShoot" "SnapToTarget" "KeepRelative" "KeepWorld" true)
                        (`KismetSystemLibrary.Delay` 0.2)
                        (`SceneComponent.SetVisibility` (`self.FakeBall`) false false)
                        (bind _returnvalue (`|SpawnActorFromClass` "/Game/bjashowdown/Blueprints/BP_Ball.BP_Ball_C" (`KismetMathLibrary.MakeTransform` (`SceneComponent.GetSocketLocation` (`self.Mesh`) "ballSocketShoot")) "Undefined" "OverrideRootScale" null null))
                        ;[1 1 1] Giving Player Access to block ball
                        (`/Game/bjashowdown/Blueprints/BP_PlyrPawn.SetBallFromAI` (`self.Plyr`) _returnvalue)
                        (bind _output_get (set `self.Ball` _returnvalue))
                        (if (or (`self.Stolen`) (`self.Blocked`))
                          (goto _label_4)
                          (else
                            (bind _outlaunchvelocity (`GameplayStatics.SuggestProjectileVelocity_CustomArc` (`self.K2_GetActorLocation` _output_get) (`self.K2_GetActorLocation` (`self.SuccessLocation`))))
                            (`ProjectileMovementComponent.SetVelocityInLocalSpace` (`/Game/bjashowdown/Blueprints/BP_Ball.ProjectileMovement` (`self.Ball`)) _outlaunchvelocity)
                            (`KismetSystemLibrary.Delay` 0.2)
                            (`SceneComponent.K2_AttachToComponent` (`self.FakeBall`) null "ballSocketR" "SnapToTarget" "KeepRelative" "KeepWorld" true)
                            ;[1 1 1] Set this to idle if you want the AI to not go after the ball after shooting
                            (`KismetSystemLibrary.Delay` 0.5)
                            (`KismetSystemLibrary.Delay` 1.0)
                            (`self.ResetShooting`)
                            (`BlackboardComponent.SetValueAsBool` (`AIBlueprintHelperLibrary.GetBlackboard` null) (`self.BallStatus`) false)
                            (bind _output_get_2 (set `self.CurrentState` "NewEnumerator7"))
                            (`self.NotifyStateChanged` _output_get_2)
                            (`KismetSystemLibrary.Delay` 0.2)
                            (`/Game/bjashowdown/AI/Opponent_AIC.EndLock` (`self.AIC`) :!label _label_6)))))))
                (else
                  (`self.ResetShooting`)
                  (set `self.CurrentState` "NewEnumerator7")))))
          (else
            (`self.ResetShooting`)
            (set `self.CurrentState` "NewEnumerator7")
            (`/Game/bjashowdown/AI/Opponent_AIC.EndLock` (`self.AIC`))))
        (elif (`/Game/bjashowdown/Blueprints/BPFL_Showdown.GetPossession` (`self.Team`))
          (bind _returnvalue_2 (`self.DecideBadShot`))
          (set `self.Bad` _returnvalue_2)
          (`KismetSystemLibrary.Delay` 0.2)
          (if (or (`self.Stolen`) (`self.Blocked`))
            (goto _label_4)
            (elif (`/Game/bjashowdown/Blueprints/BPFL_Showdown.GetPossession` (`self.Team`))
              (`/Engine/EditorBlueprintResources/StandardMacros.DoOnce` false :!label _label_7
                (:`Completed`
                  (set `self.CurrentState` "NewEnumerator4")
                  ;[1 1 1] delay set for animation/behavior tree to fire
                  (`KismetSystemLibrary.Delay` 0.2)
                  (if (or (`self.Stolen`) (`self.Blocked`))
                    (goto _label_4)
                    (elif (`KismetSystemLibrary.IsValid` _fakeball_2)
                      (`SceneComponent.K2_AttachToComponent` _fakeball_2 null "ballSocketShoot" "SnapToTarget" "KeepRelative" "KeepWorld" true)
                      (`KismetSystemLibrary.Delay` 0.2)
                      (`SceneComponent.SetVisibility` (`self.FakeBall`) false false)
                      (bind _returnvalue_3 (`|SpawnActorFromClass` "/Game/bjashowdown/Blueprints/BP_Ball.BP_Ball_C" (`KismetMathLibrary.MakeTransform` (`SceneComponent.GetSocketLocation` (`self.Mesh`) "ballSocketShoot")) "Undefined" "OverrideRootScale" null null))
                      ;[1 1 1] Giving Player Access to block ball
                      (`/Game/bjashowdown/Blueprints/BP_PlyrPawn.SetBallFromAI` (`self.Plyr`) _returnvalue_3)
                      (bind _output_get_3 (set `self.Ball` _returnvalue_3))
                      (if (or (`self.Stolen`) (`self.Blocked`))
                        (goto _label_4)
                        (else
                          (bind _outlaunchvelocity_2 (`GameplayStatics.SuggestProjectileVelocity_CustomArc` (`self.K2_GetActorLocation` _output_get_3) (`self.Bad`)))
                          (`ProjectileMovementComponent.SetVelocityInLocalSpace` (`/Game/bjashowdown/Blueprints/BP_Ball.ProjectileMovement` (`self.Ball`)) _outlaunchvelocity_2)
                          (`SceneComponent.K2_AttachToComponent` (`self.FakeBall`) null "ballSocketR" "SnapToTarget" "KeepRelative" "KeepWorld" true)
                          (`KismetSystemLibrary.Delay` 0.2)
                          ;[1 1 1] Set this to idle if you want the AI to not go after the ball after shooting
                          (`BlackboardComponent.SetValueAsBool` (`AIBlueprintHelperLibrary.GetBlackboard` null) (`self.BallStatus`) false)
                          (`KismetSystemLibrary.Delay` 1.0)
                          (`self.ResetShooting`)
                          (message `/Game/bjashowdown/Blueprints/BPI_Showdown.OnChangePossession` (`GameplayStatics.GetGameState`) "NewEnumerator2")
                          (goto _label_6)))))))
              (else
                (`self.ResetShooting`)
                (set `self.CurrentState` "NewEnumerator7")
                (`/Game/bjashowdown/AI/Opponent_AIC.EndLock` (`self.AIC`)))))
          (else
            (`self.ResetShooting`)
            (set `self.CurrentState` "NewEnumerator7")
            (`/Game/bjashowdown/AI/Opponent_AIC.EndLock` (`self.AIC`))))))))

(event `/Game/bjashowdown/Blueprints/BPI_Showdown.OnSteal`
  (params (bSuccess :type Boolean))
  (bind _bp_ball (`/Game/bjashowdown/Blueprints/BP_PlyrPawn.BP_Ball` (`self.Plyr`)))
  (`/Game/bjashowdown/Blueprints/BPFL_Showdown.LogString` (`KismetStringLibrary.Concat_StrStr` "AI OnSteal | Sucess:  " (`KismetStringLibrary.Conv_BoolToString` bSuccess)))
  (`/Game/bjashowdown/Blueprints/BPFL_Showdown.LogString` (`KismetStringLibrary.Concat_StrStr` "Player OnSteal | HasPossession:  " (`KismetStringLibrary.Conv_BoolToString` (`/Game/bjashowdown/Blueprints/BPFL_Showdown.GetPossession` (`self.Team`)))))
  (`self.LookAtPlayer`)
  (if bSuccess
    (`/Engine/EditorBlueprintResources/StandardMacros.DoOnce` false :!label _label_8
      (:`Completed`
        ;[1 1 1] Stealing
        (if (`KismetSystemLibrary.IsValid` _bp_ball)
          (`self.K2_DestroyActor` _bp_ball))
        (`SceneComponent.K2_AttachToComponent` (`self.FakeBall`) (`self.Mesh`) "ballSocketR" "SnapToTarget" "KeepRelative" "KeepWorld" true)
        (`SceneComponent.SetVisibility` (`self.FakeBall`) true false)
        (bind _output_get (set `self.CurrentState` "NewEnumerator7"))
        (`self.NotifyStateChanged` (`self.AIC`) _output_get)
        (`self.Reset`)
        (`self.LookAtGoal`)))
    (else
      (set `/Game/bjashowdown/AI/Opponent_AIC.Reset` true (`self.AIC`))
      (`self.Reset`)
      (bind _output_get_2 (set `self.CurrentState` "NewEnumerator2"))
      (`self.NotifyStateChanged` _output_get_2)
      (`KismetSystemLibrary.Delay` 1.0)
      (`/Game/bjashowdown/AI/Opponent_AIC.EndLock` (`self.AIC`)))))

(event `/Game/bjashowdown/Blueprints/BPI_Showdown.OnBlock`
  (params (bSuccess :type Boolean))
  (`/Game/bjashowdown/Blueprints/BPFL_Showdown.LogString` (`KismetStringLibrary.Concat_StrStr` "AI OnBlock | Sucess:  " (`KismetStringLibrary.Conv_BoolToString` bSuccess)))
  (`/Game/bjashowdown/Blueprints/BPFL_Showdown.LogString` (`KismetStringLibrary.Concat_StrStr` "AI OnBlock | HasPossession:  " (`KismetStringLibrary.Conv_BoolToString` (`/Game/bjashowdown/Blueprints/BPFL_Showdown.GetPossession` (`self.Team`)))))
  (if bSuccess
    (message `/Game/bjashowdown/Blueprints/BPI_Showdown.OnChangePossession` (`GameplayStatics.GetGameState`) "NewEnumerator2")
    (`/Game/bjashowdown/AI/Opponent_AIC.SetStateAsOffense` (`self.AIC`))
    (set `/Game/bjashowdown/AI/Opponent_AIC.Reset` true (`self.AIC`))
    (else
      (`KismetSystemLibrary.Delay` 5.0)
      (`/Game/bjashowdown/Blueprints/BP_PlyrPawn.SetOffensePlayer` (`self.Plyr`))
      (set `/Game/bjashowdown/AI/Opponent_AIC.Reset` true (`self.AIC`)))))

(event `Reset`
  ;[1 1 1] Reset Stealing
  (`KismetSystemLibrary.Delay` 3.0)
  (`/Game/bjashowdown/AI/Opponent_AIC.EndLock` (`self.AIC`))
  (goto _label_8 :!via `Reset`))

(event `/Game/bjashowdown/Blueprints/BPI_Showdown.OnScore`
  (params (Team :type "/Game/bjashowdown/Blueprints/Possession Enum" :default "NewEnumerator0")))

(event `/Game/bjashowdown/Blueprints/BPI_Showdown.RegisterGameObjects`
  (params (Objects :type "/Game/bjashowdown/Blueprints/S_GameObjs Structure"))
  (bind _output_get (set `self.Objects` Objects))
  (bind (_homeplayer _awayplayer _hoop _ui _aic) (break `/Game/bjashowdown/Blueprints/S_GameObjs` _output_get))
  (bind _asbp_plyr_pawn (cast `/Game/bjashowdown/Blueprints/BP_PlyrPawn` _homeplayer))
  (set `self.Plyr` _asbp_plyr_pawn)
  (bind _asopponent_aic (cast `/Game/bjashowdown/AI/Opponent_AIC` _aic))
  (set `self.AIC` _asopponent_aic)
  (bind _asbp_hoop (cast `/Game/bjashowdown/Blueprints/BP_Hoop` _hoop))
  (set `self.H00p` _asbp_hoop))

(event `SetStolen`
  (set `self.Stolen` true))

(event `SetBlocked`
  (set `self.Blocked` true))

(event `/Game/bjashowdown/Blueprints/BPI_Showdown.OnChangePossession`
  (params (Possession :type "/Game/bjashowdown/Blueprints/Possession Enum" :default "NewEnumerator0"))
  (if (`|EnumEquality` Possession (`self.Team`))
    (`SceneComponent.SetVisibility` (`self.FakeBall`) true true)))

(fn `AttemptAction`
  (params (Team :type "/Game/bjashowdown/Blueprints/Possession Enum" :default "NewEnumerator0") (ActionTaken :type "/Game/bjashowdown/Blueprints/PlayerActions Enum" :default "NewEnumerator0"))
  (return))

(fn `DecideBadShot`
  (returns (ReturnValue :type "Vector Structure"))
  (bind _getbadlocation (`self.GetHoopLocation`))
  (return (`KismetMathLibrary.TransformLocation` (`self.GetTransform` _getbadlocation) (`|GetArrayItem` (`/Game/bjashowdown/Shared/HoopLocationBase.ShotPoint` _getbadlocation) (`KismetMathLibrary.RandomInteger` 3)))))

(fn `GetHoopLocation`
  (returns (GetBadLocation :type "/Game/bjashowdown/Shared/HoopLocationBase Object Reference"))
  (return (`self.HoopShotLocation`)))

(fn `GetIsIdle`
  (returns (Idle :type "/Game/bjashowdown/Blueprints/NPC_State Enum"))
  (return "NewEnumerator0"))

(fn `GetShotLocation`
  (returns (Location :type "/Game/bjashowdown/AI/ShotLocationBase Object Reference"))
  (return (`self.MyShotLocation`)))

(fn `GetSuccessShotLocation`
  (returns (SuccessShotBase :type "/Game/bjashowdown/Shared/SuccessShotBase Object Reference"))
  (return null))

(fn `GetTeamID`
  (returns (IsPlayer :type Boolean))
  (return false))

(fn `OnGameEvent`
  (params (Event :type "/Game/bjashowdown/Blueprints/GameEvent Enum" :default "NewEnumerator0"))
  (`/Game/bjashowdown/Blueprints/BPFL_Showdown.LogString` (`KismetStringLibrary.Concat_StrStr` "AI GameEvent ||" (`|GetEnumeratorNameAsString` Event)))
  (switch `/Game/bjashowdown/Blueprints/GameEvent` (`local.Event`)
    (:`NewEnumerator1`
      ;[1 1 1] TODO: move to start pos
      (`/Game/bjashowdown/Blueprints/BPFL_Showdown.LogString` "AI | Move to Start Pos")
      (`self.MoveToStartPos`)
      (return))
    (:`NewEnumerator2`
      (`self.OnCheckBall`)
      (return))
    (:`NewEnumerator4`
      (if (`/Game/bjashowdown/Blueprints/BPFL_Showdown.GetPossession` (`self.Team`))
        (set `self.ActionStatus` (make `/Game/bjashowdown/Blueprints/S_Actions` true false true))
        (else
          (set `self.ActionStatus` (make `/Game/bjashowdown/Blueprints/S_Actions` false true true))))
      (return))))

(fn `UserConstructionScript`)