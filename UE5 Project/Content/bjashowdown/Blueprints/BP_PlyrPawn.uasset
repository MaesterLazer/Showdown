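; Player pawn for a one-on-one basketball game against an AI opponent, driven by a touch joystick and a tap zone.
; The tap sends a shoot, steal or block attempt to the game state by possession and proximity, and result events update animation states and both players.
; Shots swap the socketed fake ball for a projectile launched on a suggested arc; blocked shots spawn a physics ball, and overlapping one grants possession.
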(event `self.ReceiveBeginPlay`
  (bind _shootblock (`self.ShootBlock`))
  (`|ExecutionSequence`
    (:`then_0`
      (set `self.Stats` (make `/Game/bjashowdown/Blueprints/S_Stats` (`KismetMathLibrary.RandomFloatInRange` 0.0 1.0) (`KismetMathLibrary.RandomFloatInRange` 0.0 1.0) (`KismetMathLibrary.RandomFloatInRange` 0.0 1.0) (`KismetMathLibrary.RandomFloatInRange` 0.0 1.0))))
    (:`then_1`
      (`/Game/UltimateTouchComponents/Core/UTCJoystickComponent.Setup Widget` (`self.MoveJoy`) (`self.JoyWidget`) true true)
      (set `self.CurrentState` "NewEnumerator0")
      (`self.NotifyStateChanged` "NewEnumerator0")
      (`self.GetIsIdle`))
    (:`then_2`
      (`/Game/UltimateTouchComponents/Core/UTCComponent.Setup Bounds` _shootblock true (0.8 0.7) (0.0 0.2) true true)
      (`/Game/UltimateTouchComponents/Core/UTCComponent.Setup Background by Bounds` _shootblock (`self.ShootBlockWidget`) true)
      (`UserWidget.SetColorAndOpacity` (`/Game/UltimateTouchComponents/Core/UTCComponent.Background Widget` (`self.ShootBlock`)) (struct :`R` 1.0 :`G` 1.0 :`B` 1.0 :`A` 0.45)))))

(event `InputTouch`
  (params (Location :type "Vector Structure") (FingerIndex :type "ETouchIndex Enum"))
  ;[1 0 0] Pass required events to all UTC components
  (:`Pressed`
    (`/Game/UltimateTouchComponents/Core/UTCMacroLibrary.UTC Touch Input Manager` Location FingerIndex :!label _label))
  (:`Released`
    (goto _label :!via `Released`))
  (:`Moved`
    (goto _label :!via `Moved`)))

(event `self.ReceivePossessed`
  (params (NewController :type "Controller Object Reference"))
  ;[1 0 0] Pass required events to all UTC components
  (`/Game/UltimateTouchComponents/Core/UTCMacroLibrary.UTC Pawn Possesion Manager` NewController (stale `self.ReceiveUnpossessed` OldController) :!label _label_2))

(event `self.ReceiveUnpossessed`
  (params (OldController :type "Controller Object Reference"))
  ;[1 0 0] Pass required events to all UTC components
  (goto _label_2 :!via `Unpossesed`))

(event `self.MoveJoy.On X Axis Changed`
  (params (Value :type "Float (single-precision)"))
  (bind _oppo (`self.Oppo`))
  ;[0 1 0] Movement
  (if (not (`NavMovementComponent.IsFalling` (`self.CharacterMovement`)))
    (`self.AddMovementInput` (0.0 1.0 0.0) (* Value 1.0))
    (bind _output_get (set `self.CurrentState` "NewEnumerator1" :!label _label_3))
    (`self.NotifyStateChanged` _output_get)
    (`self.GetIsIdle`)
    (`KismetSystemLibrary.Delay` 0.2)
    (if (`/Game/bjashowdown/Blueprints/BPFL_Showdown.GetPossession` (`self.Team`))
      (bind _output_get_2 (set `self.CurrentState` "NewEnumerator6"))
      (`self.NotifyStateChanged` _output_get_2)
      (`self.GetIsIdle`)
      (set `/Game/bjashowdown/Blueprints/BP_Opponent.CurrentState` "NewEnumerator0" _oppo)
      (`/Game/bjashowdown/Blueprints/BP_Opponent.NotifyStateChanged` _oppo "NewEnumerator0"))))

(event `self.MoveJoy.On Y Axis Changed`
  (params (Value :type "Float (single-precision)"))
  ;[0 1 0] Movement
  (if (not (`NavMovementComponent.IsFalling` (`self.CharacterMovement`)))
    (`self.AddMovementInput` (1.0 0.0 0.0) Value)
    (goto _label_3)))

(event `/Game/bjashowdown/Blueprints/BPI_Showdown.RegisterGameObjects`
  (params (Objects :type "/Game/bjashowdown/Blueprints/S_GameObjs Structure"))
  (bind _output_get (set `self.GameObjs` Objects))
  (bind (_homeplayer _awayplayer _hoop _ui _aic) (break `/Game/bjashowdown/Blueprints/S_GameObjs` _output_get))
  (bind _asbp_opponent (cast `/Game/bjashowdown/Blueprints/BP_Opponent` _awayplayer))
  (set `self.Oppo` _asbp_opponent)
  (bind _asopponent_aic (cast `/Game/bjashowdown/AI/Opponent_AIC` _aic))
  (set `self.Aic` _asopponent_aic))

(event `self.CapsuleComponent.OnComponentBeginOverlap`
  (params (OverlappedComponent :type "PrimitiveComponent Object Reference") (OtherActor :type "Actor Object Reference") (OtherComp :type "PrimitiveComponent Object Reference") (OtherBodyIndex :type Integer) (bFromSweep :type Boolean) (SweepResult :type "HitResult Structure (by ref)"))
  (bind _returnvalue (`self.K2_GetActorLocation` (`/Game/bjashowdown/Blueprints/BP_Opponent.H00p` (`self.Oppo`))))
  (bind _returnvalue_2 (- (`self.K2_GetActorLocation`) _returnvalue))
  (bind _asbp_fake_ball (cast `/Game/bjashowdown/Blueprints/BP_FakeBall` OtherActor))
  (if (`KismetSystemLibrary.IsValid` _asbp_fake_ball)
    (message `/Game/bjashowdown/Blueprints/BPI_Showdown.OnChangePossession` (`GameplayStatics.GetGameState`) "NewEnumerator0")
    (`self.setballforaic` _asbp_fake_ball)
    (set `self.CurrentState` "NewEnumerator6")
    (`self.GetIsIdle`)
    (`SceneComponent.SetVisibility` (`self.FakeBall`) true false)
    (`self.K2_DestroyActor` _asbp_fake_ball)
    (`BlackboardComponent.SetValueAsVector` (`AIBlueprintHelperLibrary.GetBlackboard` (`self.Aic`)) (`self.Moveto`) (+ _returnvalue (* (`KismetMathLibrary.Normal` _returnvalue_2) (* (`KismetMathLibrary.VSize` _returnvalue_2) 50.0))))))

(event `self.ShootBlock.On Tap`
  (params (Location :type "Vector Structure") (FingerIndex :type "ETouchIndex Enum" :default "Touch1"))
  (`UserWidget.SetColorAndOpacity` (`/Game/UltimateTouchComponents/Core/UTCComponent.Background Widget` (`self.ShootBlock`)) (struct :`R` 1.0 :`G` 1.0 :`B` 1.0 :`A` 1.0))
  (`self.OnShoot` :!label _label_4)
  (bind _output_get (set `self.CurrentState` "NewEnumerator4"))
  (`self.NotifyStateChanged` _output_get)
  (`self.GetIsIdle`))

(event `self.ShootBlock.On Tap Release`
  (params (Location :type "Vector Structure") (FingerIndex :type "ETouchIndex Enum" :default "Touch1"))
  (`UserWidget.SetColorAndOpacity` (`/Game/UltimateTouchComponents/Core/UTCComponent.Background Widget` (`self.ShootBlock`)) (struct :`R` 1.0 :`G` 1.0 :`B` 1.0 :`A` 0.45))
  (goto _label_4))

(event `OnShoot`
  (if (`/Game/bjashowdown/Blueprints/BPFL_Showdown.GetPossession` (`self.Team`)) :!label _label_5
    (message `/Game/bjashowdown/Blueprints/BPI_Showdown.AttemptAction` (`GameplayStatics.GetGameState`) "NewEnumerator0" "NewEnumerator0")
    (elif (== (`SceneComponent.K2_GetComponentLocation` (`self.StealSphere`)) (`self.K2_GetActorLocation` (`self.Oppo`)) :`ErrorTolerance` 100.0)
      (if (`/Game/bjashowdown/Blueprints/BPFL_Showdown.GetPossession` (`/Game/bjashowdown/Blueprints/BP_Opponent.Team` (`self.Oppo`)))
        (message `/Game/bjashowdown/Blueprints/BPI_Showdown.AttemptAction` (`GameplayStatics.GetGameState`) "NewEnumerator0" "NewEnumerator2"))
      (else
        (message `/Game/bjashowdown/Blueprints/BPI_Showdown.AttemptAction` (`GameplayStatics.GetGameState`) "NewEnumerator0" "NewEnumerator1")))))

(event `Key|S`
  (params (Key :type "Key Structure"))
  (:`Pressed`
    (goto _label_5)))

(event `SetBallFromAI`
  (params (BallAI :type "/Game/bjashowdown/Blueprints/BP_Ball Object Reference"))
  ;[1 1 1] Setting the ball from AI
  (set `self.BP_Ball` BallAI))

(event `BallGone`
  ;[1 1 1] Stolen
  (`SceneComponent.SetVisibility` (`self.FakeBall`) false false)
  (bind _output_get (set `self.CurrentState` "NewEnumerator0"))
  (`self.NotifyStateChanged` _output_get))

(event `setballforaic`
  (params (Ball :type "/Game/bjashowdown/Blueprints/BP_FakeBall Object Reference (by ref)"))
  ;[1 1 1] This sets the ball after hoop destroys it for AI
  (set `self.BP_Faker` Ball))

(event `/Game/bjashowdown/Blueprints/BPI_Showdown.OnGameplayEvent`
  (params (Event :type "/Game/bjashowdown/Blueprints/GameEvent Enum" :default "NewEnumerator0"))
  (`self.ReceiveGameEvent` Event))

(event `MoveToStartPos`
  (`KismetSystemLibrary.Delay` 0.2)
  (message `/Game/bjashowdown/Blueprints/BPI_Showdown.ReadyUp` (`GameplayStatics.GetGameState`) (`self.Team`)))

(event `OnCheckBall`
  (bind _bhaspossession (`/Game/bjashowdown/Blueprints/BPFL_Showdown.GetPossession` (`self.Team`)))
  (`/Game/bjashowdown/Blueprints/BPFL_Showdown.LogString` (`KismetStringLibrary.Concat_StrStr` "Player CheckBall | HasPossession:  " (`KismetStringLibrary.Conv_BoolToString` _bhaspossession)))
  (if _bhaspossession
    _))

(event `/Game/bjashowdown/Blueprints/BPI_Showdown.OnShootBasket`
  (params (bSuccess :type Boolean))
  (bind _oppo (`self.Oppo`))
  (bind _hooplocationbase (`self.HoopLocationBase`))
  (`/Game/bjashowdown/Blueprints/BPFL_Showdown.LogString` (`KismetStringLibrary.Concat_StrStr` "Player OnShoot | Sucess:  " (`KismetStringLibrary.Conv_BoolToString` bSuccess)))
  (`/Game/bjashowdown/Blueprints/BPFL_Showdown.LogString` (`KismetStringLibrary.Concat_StrStr` "Player OnShoot | HasPossession:  " (`KismetStringLibrary.Conv_BoolToString` (`/Game/bjashowdown/Blueprints/BPFL_Showdown.GetPossession` (`self.Team`)))))
  (if bSuccess
    (set `self.CurrentState` "NewEnumerator4")
    (`self.GetIsIdle`)
    (`self.LookAtGoal`)
    (`self.Jump`)
    (`SceneComponent.K2_AttachToComponent` (`self.FakeBall`) null (`self.ShootSocket`) "SnapToTarget" "KeepRelative" "KeepWorld" true)
    (`KismetSystemLibrary.Delay` 0.49)
    (`SceneComponent.SetVisibility` (`self.FakeBall`) false false)
    (bind _returnvalue (`|SpawnActorFromClass` "/Game/bjashowdown/Blueprints/BP_Ball.BP_Ball_C" (`KismetMathLibrary.MakeTransform` (`SceneComponent.GetSocketLocation` (`self.Mesh`) "None")) "Undefined" "OverrideRootScale" null null))
    (bind _output_get (set `self.BP_Ball` _returnvalue))
    (bind _outlaunchvelocity (`GameplayStatics.SuggestProjectileVelocity_CustomArc` (`self.K2_GetActorLocation` _output_get) (`self.K2_GetActorLocation` (`self.SuccessShotBase`))))
    (`ProjectileMovementComponent.SetVelocityInLocalSpace` (`/Game/bjashowdown/Blueprints/BP_Ball.ProjectileMovement` (`self.BP_Ball`)) _outlaunchvelocity)
    ;[1 1 1] This is here to enable AI to actually be able to block
    (`KismetSystemLibrary.Delay` 0.3)
    (message `/Game/bjashowdown/Blueprints/BPI_Showdown.OnChangePossession` (`GameplayStatics.GetGameState`) "NewEnumerator2")
    (`self.EnableInput` self (`GameplayStatics.GetPlayerController` 0) :!label _label_6)
    (`SceneComponent.K2_AttachToComponent` (`self.FakeBall`) null (`self.DribbleSocket`) "SnapToTarget" "KeepRelative" "KeepWorld" true)
    (bind _output_get_2 (set `self.CurrentState` "NewEnumerator7"))
    (`self.NotifyStateChanged` _output_get_2)
    (`KismetSystemLibrary.Delay` 0.2)
    (bind _output_get_3 (set `/Game/bjashowdown/Blueprints/BP_Opponent.CurrentState` "NewEnumerator7" _oppo))
    (`/Game/bjashowdown/Blueprints/BP_Opponent.NotifyStateChanged` _oppo _output_get_3)
    (elif (`/Game/bjashowdown/Blueprints/BPFL_Showdown.GetPossession` (`self.Team`))
      (set `self.CurrentState` "NewEnumerator4")
      (`self.GetIsIdle`)
      (`self.LookAtGoal`)
      (`self.Jump`)
      (`SceneComponent.K2_AttachToComponent` (`self.FakeBall`) null (`self.ShootSocket`) "SnapToTarget" "KeepRelative" "KeepWorld" true)
      (`KismetSystemLibrary.Delay` 0.49)
      (`SceneComponent.SetVisibility` (`self.FakeBall`) false false)
      (bind _returnvalue_2 (`|SpawnActorFromClass` "/Game/bjashowdown/Blueprints/BP_Ball.BP_Ball_C" (`KismetMathLibrary.MakeTransform` (`SceneComponent.GetSocketLocation` (`self.Mesh`) "None")) "Undefined" "OverrideRootScale" null null))
      (bind _output_get_4 (set `self.BP_Ball` _returnvalue_2))
      (bind _outlaunchvelocity_2 (`GameplayStatics.SuggestProjectileVelocity_CustomArc` (`self.K2_GetActorLocation` _output_get_4) (`KismetMathLibrary.TransformLocation` (`self.GetTransform` _hooplocationbase) (`|GetArrayItem` (`/Game/bjashowdown/Shared/HoopLocationBase.ShotPoint` _hooplocationbase) (`KismetMathLibrary.RandomInteger` 3)))))
      (`ProjectileMovementComponent.SetVelocityInLocalSpace` (`/Game/bjashowdown/Blueprints/BP_Ball.ProjectileMovement` (`self.BP_Ball`)) _outlaunchvelocity_2)
      ;[1 1 1] This is here to enable AI to actually be able to block
      (`KismetSystemLibrary.Delay` 0.3)
      (message `/Game/bjashowdown/Blueprints/BPI_Showdown.OnChangePossession` (`GameplayStatics.GetGameState`) "NewEnumerator2")
      (goto _label_6))))

(event `/Game/bjashowdown/Blueprints/BPI_Showdown.OnSteal`
  (params (bSuccess :type Boolean))
  (`/Game/bjashowdown/Blueprints/BPFL_Showdown.LogString` (`KismetStringLibrary.Concat_StrStr` "Player OnSteal | Sucess:  " (`KismetStringLibrary.Conv_BoolToString` bSuccess)))
  (`/Game/bjashowdown/Blueprints/BPFL_Showdown.LogString` (`KismetStringLibrary.Concat_StrStr` "Player OnSteal | HasPossession:  " (`KismetStringLibrary.Conv_BoolToString` (`/Game/bjashowdown/Blueprints/BPFL_Showdown.GetPossession` (`self.Team`)))))
  (if bSuccess
    (bind _output_get (set `self.CurrentState` "NewEnumerator3"))
    (`self.NotifyStateChanged` _output_get)
    (`/Game/bjashowdown/Blueprints/BP_Opponent.PlayerStole` (`self.Oppo`))
    (message `/Game/bjashowdown/Blueprints/BPI_Showdown.OnChangePossession` (`GameplayStatics.GetGameState`) "NewEnumerator0")
    (`SceneComponent.K2_AttachToComponent` (`self.FakeBall`) null "ballSocketR" "SnapToTarget" "KeepRelative" "KeepWorld" true)
    (`SceneComponent.SetVisibility` (`self.FakeBall`) true false)
    (bind _output_get_2 (set `self.CurrentState` "NewEnumerator0"))
    (`/Game/bjashowdown/Blueprints/BP_Opponent.NotifyStateChanged` _output_get_2)))

(event `/Game/bjashowdown/Blueprints/BPI_Showdown.OnBlock`
  (params (bSuccess :type Boolean))
  (bind _oppo (`self.Oppo`))
  (`/Game/bjashowdown/Blueprints/BPFL_Showdown.LogString` (`KismetStringLibrary.Concat_StrStr` "Player OnBlock | Sucess:  " (`KismetStringLibrary.Conv_BoolToString` bSuccess)))
  (if bSuccess
    (bind _output_get (set `self.CurrentState` "NewEnumerator9"))
    (`self.NotifyStateChanged` _output_get)
    (else
      (bind _output_get_2 (set `self.CurrentState` "NewEnumerator2"))
      (`self.NotifyStateChanged` _output_get_2)))
  (if bSuccess
    (`/Game/bjashowdown/Blueprints/BP_Opponent.Blocked` _oppo))
  (`KismetSystemLibrary.Delay` 0.2)
  (bind _output_get_3 (set `/Game/bjashowdown/Blueprints/BP_Opponent.CurrentState` "NewEnumerator7" _oppo))
  (`/Game/bjashowdown/Blueprints/BP_Opponent.NotifyStateChanged` _oppo _output_get_3))

(event `SetOffensePlayer`
  (bind _output_get (set `self.CurrentState` "NewEnumerator7"))
  (`self.NotifyStateChanged` _output_get))

(event `Blocked`
  (bind _bp_ball (`self.BP_Ball`))
  ;[1 1 1] Possession changed in oppo
  ;[1 1 1] Ball Blocked
  ;;[1 1 1] can't be higher than .5
  (`KismetSystemLibrary.Delay` 0.5)
  (`ProjectileMovementComponent.SetVelocityInLocalSpace` (`/Game/bjashowdown/Blueprints/BP_Ball.ProjectileMovement` _bp_ball) (`KismetMathLibrary.MakeVector` (`KismetMathLibrary.RandomFloatInRange` -80.0 80.0)))
  (`/Engine/EditorBlueprintResources/StandardMacros.DoOnce` false
    (:`Completed`
      (bind _returnvalue (`|SpawnActorFromClass` "/Game/bjashowdown/Blueprints/BP_FakeBall.BP_FakeBall_C" (`self.GetTransform` _bp_ball) "Undefined" "OverrideRootScale" null null))
      (`PrimitiveComponent.SetSimulatePhysics` (`/Game/bjashowdown/Blueprints/BP_FakeBall.Main` _returnvalue) true)
      (set `self.BP_Faker` _returnvalue))))

(event `/Game/bjashowdown/Blueprints/BPI_Showdown.OnScore`
  (params (Team :type "/Game/bjashowdown/Blueprints/Possession Enum" :default "NewEnumerator0"))
  ;[1 1 1] Scoring
)

(fn `AttemptAction`
  (params (Team :type "/Game/bjashowdown/Blueprints/Possession Enum" :default "NewEnumerator0") (ActionTaken :type "/Game/bjashowdown/Blueprints/PlayerActions Enum" :default "NewEnumerator0"))
  (return))

(fn `GetHoopLocation`
  (returns (GetBadLocation :type "/Game/bjashowdown/Shared/HoopLocationBase Object Reference"))
  (return null))

(fn `GetIsIdle`
  (returns (Idle :type "/Game/bjashowdown/Blueprints/NPC_State Enum"))
  (return (`self.CurrentState`)))

(fn `GetShotLocation`
  (returns (Location :type "/Game/bjashowdown/AI/ShotLocationBase Object Reference"))
  (return null))

(fn `GetSuccessShotLocation`
  (returns (SuccessShotBase :type "/Game/bjashowdown/Shared/SuccessShotBase Object Reference"))
  (return null))

(fn `GetTeamID`
  (returns (IsPlayer :type Boolean))
  (return true))

(fn `ReceiveGameEvent`
  (params (Event :type "/Game/bjashowdown/Blueprints/GameEvent Enum" :default "NewEnumerator0"))
  (`/Game/bjashowdown/Blueprints/BPFL_Showdown.LogString` (`KismetStringLibrary.Concat_StrStr` "Player GameEvent ||" (`|GetEnumeratorNameAsString` Event)))
  (switch `/Game/bjashowdown/Blueprints/GameEvent` (`local.Event`)
    (:`NewEnumerator1`
      ;[1 1 1] TODO: move to start pos
      (`/Game/bjashowdown/Blueprints/BPFL_Showdown.LogString` "Player | Move to Start Pos")
      (`self.MoveToStartPos`)
      (return))
    (:`NewEnumerator2`
      (`self.OnCheckBall`)
      (return))
    (:`NewEnumerator4`
      (if (`/Game/bjashowdown/Blueprints/BPFL_Showdown.GetPossession` (`self.Team`))
        (set `self.ActionStatus` (make `/Game/bjashowdown/Blueprints/S_Actions` true false true))
        (else
          (set `self.ActionStatus` (make `/Game/bjashowdown/Blueprints/S_Actions` false true true))))
      (return))))

(fn `UserConstructionScript`
  (`SceneComponent.K2_AttachToComponent` (`self.FakeBall`) (`self.Mesh`) "ballsocketR" "SnapToTarget" "KeepRelative" "KeepWorld" true))