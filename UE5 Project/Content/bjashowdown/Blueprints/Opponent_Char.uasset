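; AI opponent character for a basketball game that picks up, steals and shoots the ball.
; State changes are forwarded to the anim instance; overlapping a loose fake ball while the player lacks possession grants possession and updates the blackboard.
; A steal runs a once-only timed jump shot, swapping the socketed fake ball for a spawned BP_Ball arced toward the blackboard hoop location.
; Player steals clear possession; successful blocks trigger a delayed state change.
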(event `self.ReceiveBeginPlay`)

(event `self.NotifyStateChanged`
  (params (NewState :type "/Game/bjashowdown/AI/NPC_State Enum" :default "NewEnumerator0"))
  ;[1 1 1] State Updates
  (bind _output_get (set `self.CurrentState` NewState))
  (message `/Game/bjashowdown/Shared/BPI_AI_Helper.NotifyStateChanged` (`SkeletalMeshComponent.GetAnimInstance` (`self.Mesh`)) _output_get))

(event `Stealing`
  ;[1 1 1] Stealing
  (set `self.Stolen` true)
  (`/Engine/EditorBlueprintResources/StandardMacros.DoOnce` false :!label _label
    (:`Completed`
      (`SceneComponent.K2_AttachToComponent` (`self.FakeBall`) (`self.Mesh`) "ballSocketR" "SnapToTarget" "KeepRelative" "KeepWorld" true)
      (`SceneComponent.SetVisibility` (`self.FakeBall`) true false)
      (`KismetSystemLibrary.Delay` 0.5)
      (`self.Jump`)
      (`SceneComponent.K2_AttachToComponent` (`self.FakeBall`) null "ballSocketShoot" "SnapToTarget" "KeepRelative" "KeepWorld" true)
      (`KismetSystemLibrary.Delay` 0.49)
      (`SceneComponent.SetVisibility` (`self.FakeBall`) false false)
      (bind _returnvalue (`|SpawnActorFromClass` "/Game/bjashowdown/Blueprints/BP_Ball.BP_Ball_C" (`KismetMathLibrary.MakeTransform` (`SceneComponent.GetSocketLocation` (`self.Mesh`) "ballSocketShoot")) "Undefined" "OverrideRootScale" null null))
      (bind _output_get (set `self.Ball` _returnvalue))
      (bind _outlaunchvelocity (`GameplayStatics.SuggestProjectileVelocity_CustomArc` (`self.K2_GetActorLocation` _output_get) (`BlackboardComponent.GetValueAsVector` (`AIBlueprintHelperLibrary.GetBlackboard` (`AIBlueprintHelperLibrary.GetAIController` self)) (`self.HoopLoc`))))
      (`ProjectileMovementComponent.SetVelocityInLocalSpace` (`/Game/bjashowdown/Blueprints/BP_Ball.ProjectileMovement` (`self.Ball`)) _outlaunchvelocity)
      (`SceneComponent.K2_AttachToComponent` (`self.FakeBall`) null "ballSocketR" "SnapToTarget" "KeepRelative" "KeepWorld" true)
      (set `self.Possession` false)
      (`KismetSystemLibrary.Delay` 0.5)
      ;[1 1 1] Current State is Idle -- will be changed to offense after it is implemented
      (bind _output_get_2 (set `self.CurrentState` "NewEnumerator7"))
      (`self.NotifyStateChanged` _output_get_2))))

(event `SuccessfullyBlocked`
  ;[1 1 1] Blocking change over
  (`KismetSystemLibrary.Delay` 1.0)
  ;;[1 1 1] Current State is Idle -- will be changed to offense after it is implemented
  (bind _output_get (set `self.CurrentState` "NewEnumerator7"))
  (`self.NotifyStateChanged` _output_get))

(event `Reset`
  (`KismetSystemLibrary.Delay` 1.0)
  (goto _label :!via `Reset`))

(event `self.CapsuleComponent.OnComponentBeginOverlap`
  (params (OverlappedComponent :type "PrimitiveComponent Object Reference") (OtherActor :type "Actor Object Reference") (OtherComp :type "PrimitiveComponent Object Reference") (OtherBodyIndex :type Integer) (bFromSweep :type Boolean) (SweepResult :type "HitResult Structure (by ref)"))
  (`KismetSystemLibrary.Delay` 1.0)
  (bind _asbp_plyr_pawn (cast `/Game/bjashowdown/Blueprints/BP_PlyrPawn` (`GameplayStatics.GetPlayerPawn` 0)))
  (if (not (`/Game/bjashowdown/Blueprints/BP_PlyrPawn.bPossession` _asbp_plyr_pawn))
    (bind _asbp_fake_ball (cast `/Game/bjashowdown/Blueprints/BP_FakeBall` OtherActor))
    (if (`KismetSystemLibrary.IsValid` _asbp_fake_ball)
      (bind _output_get (set `self.Possession` true))
      (`BlackboardComponent.SetValueAsBool` (`AIBlueprintHelperLibrary.GetBlackboard` null) (`self.BallStatus`) _output_get)
      (`SceneComponent.K2_AttachToComponent` (`self.FakeBall`) (`self.Mesh`) "ballSocketR" "SnapToTarget" "KeepRelative" "KeepWorld" true)
      (`SceneComponent.SetVisibility` (`self.FakeBall`) true false)
      (`self.K2_DestroyActor` OtherActor)
      (set `self.CurrentState` "NewEnumerator7"))))

(event `PlayerStole`
  ;[1 1 1] For when the Player steals the ball from AI
  (set `self.Possession` false)
  (`SceneComponent.SetVisibility` (`self.FakeBall`) false false))

(fn `GetIsIdle`
  (returns (Idle :type "/Game/bjashowdown/AI/NPC_State Enum"))
  (return "NewEnumerator0"))

(fn `GetTeamID`
  (returns (IsPlayer :type Boolean))
  (return false))

(fn `UserConstructionScript`)